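; Interactable elevator with a rotating windlass that travels between its initial transform and a destination point.
; On the server, each interaction runs the travel forward or backward based on the interactable value, then changes that value.
; Travel updates lerp the actor transform and windlass rotation, with a RepNotify applying the spin to the mesh.
; The timeline position is stored in the interactable component and restored on game load.
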(event `/Game/RPG_InventorySystem/Blueprints/BPI_Interactable.Interaction`
  (params (Interactor :type "Actor Object Reference"))
  ;[0 0 0 0.227 22] SERVER: On Interaction
  (`/Engine/EditorBlueprintResources/StandardMacros.IsValid` Interactor
    (:`Is Valid`
      (bind _output_get (set `self.Interactor` Interactor))
      (`self.SetOwner` _output_get)
      (`|ExecutionSequence`
        (:`then_0`
          (switch `int` (`/Game/RPG_InventorySystem/Blueprints/Components/AC_Interactable.Interactable Value` (`self.AC_Interactable`))
            (:`0`
              (`self.Move Forward`))
            (:`1`
              (`self.Move Backward`))))
        (:`then_1`
          (`/Game/RPG_InventorySystem/Blueprints/Components/AC_Interactable.Change Interactable Value` (`self.AC_Interactable`) true))))))

(event `/Game/RPG_InventorySystem/Blueprints/BPI_Interactable.Initialize`
  ;[0 0 0 0.227 22] On Initialize
  (`/Game/RPG_InventorySystem/Blueprints/Components/AC_Interactable.Setup Interactable References` (`self.AC_Interactable`) (`self.InteractableArea`) (`self.InteractionWidget`) (`|MakeSet` (`self.Windlass`) :!type "PrimitiveComponent Object Reference")))

(event `/Game/RPG_InventorySystem/Blueprints/BPI_Interactable.End Interaction`
  (params (Interactor :type "Actor Object Reference"))
  ;[0 0 0 0.227 22] On End Interaction
)

(event `/Game/RPG_InventorySystem/Blueprints/BPI_Interactable.Remove Interaction`
  ;[0 0 0 0.227 22] On Remove Interaction
)

(event `/Game/RPG_InventorySystem/Blueprints/BPI_Interactable.Game Load`
  ;[0 0 0 0.227 22] On Game Load
  (`self.Set Timeline Postion` (`/Game/RPG_InventorySystem/Blueprints/Components/AC_Interactable.Timeline Position` (`self.AC_Interactable`))))

(fn `OnRep_Windlass Rotation`
  (`SceneComponent.K2_SetRelativeRotation` (`self.Windlass`) (`self.Windlass Rotation`) false false))

(fn `Travel Finished`
  (`parent.Travel Finished`))

(fn `Update Travel Transform`
  (params (`Current Time` :type "Float (double-precision)"))
  (bind _destination_point (`/Game/RPG_InventorySystem/Blueprints/Components/AC_Interactable.Destination Point` (`self.AC_Interactable`)))
  (`/Engine/EditorBlueprintResources/StandardMacros.IsValid` _destination_point
    (:`Is Valid`
      (`self.K2_SetActorTransform` (`KismetMathLibrary.TLerp` (`self.Initial Transform`) (`self.GetTransform` _destination_point) `Current Time`))
      (set `self.Windlass Rotation` (`KismetMathLibrary.RLerp` (struct :`Yaw` 180.0) (`KismetMathLibrary.MakeRotator` (* (`self.Rotation Amount`) 360.0) 0.0 180.0) `Current Time`))
      (set `/Game/RPG_InventorySystem/Blueprints/Components/AC_Interactable.Timeline Position` (`TimelineComponent.GetPlaybackPosition` (`self.Timeline_ObjectTransform`)) (`self.AC_Interactable`)))))

(fn `UserConstructionScript`)