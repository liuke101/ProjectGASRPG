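; Elevator winch that visually spins and holds a rope attached to a linked movable object, MainMovableRef.
; On BeginPlay it binds to that object's move forward, move backward, finished and stop events.
; A single timeline drives the mesh's roll, playing on backward movement, reversing on forward movement and stopping when movement ends.
; The construction script attaches the rope's end to the movable's CableEnd component.
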(event `self.ReceiveBeginPlay`
  ;[0.05347 1 0 0.493] Bind Movable Object Events
  (`/Engine/EditorBlueprintResources/StandardMacros.IsValid` (`self.Main Movable Ref`)
    (:`Is Valid`
      (add `/Game/RPG_InventorySystem/Classes/Interactable/Miscellaneous/BP_MainMovableObject.On Move Forward` (`self.Main Movable Ref`) (`|CreateDelegate` :!event `On Move Forward`))
      (add `/Game/RPG_InventorySystem/Classes/Interactable/Miscellaneous/BP_MainMovableObject.On Move Backward` (`self.Main Movable Ref`) (`|CreateDelegate` :!event `On Move Backward`))
      (add `/Game/RPG_InventorySystem/Classes/Interactable/Miscellaneous/BP_MainMovableObject.On Moving Finished` (`self.Main Movable Ref`) (`|CreateDelegate` :!event `Stop Moving`))
      (add `/Game/RPG_InventorySystem/Classes/Interactable/Miscellaneous/BP_MainMovableObject.On Stop Moving` (`self.Main Movable Ref`) (`|CreateDelegate` :!event `Stop Moving`)))))

(event `On Move Backward`
  ;[1 0.04186 0 0.546] Rotate Winch
  (bind (_direction _rotationx) (`Timeline|Timeline_Rotation` :!label _label)
    (:`Update`
      (`SceneComponent.K2_SetRelativeRotation` (`self.StaticMesh`) (`KismetMathLibrary.MakeRotator` (.x _rotationx)) false false))))

(event `Stop Moving`
  ;[1 0.04186 0 0.546] Rotate Winch
  (goto _label :!via `Stop`))

(event `On Move Forward`
  ;[1 0.04186 0 0.546] Rotate Winch
  (goto _label :!via `Reverse`))

(fn `UserConstructionScript`
  (bind _main_movable_ref (`self.Main Movable Ref`))
  (`/Engine/EditorBlueprintResources/StandardMacros.IsValid` _main_movable_ref
    (:`Is Valid`
      (`CableComponent.SetAttachEndTo` (`self.Rope`) _main_movable_ref "CableEnd" "None"))))