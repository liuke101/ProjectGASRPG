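; BP_TriggerType01 is an interactable trigger whose lever slides down or back up, alternating with the ACInteractable component's interactable value.
; Interaction sets the interactor as owner, moves the lever, updates that value and notifies associated actors through the component.
; A timeline drives LeverLocation, whose OnRep applies the relative location, and can reinitialize the component when finished.
; Timeline position and direction are stored on the component to resume movement after unpause or game load.
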(event `/Game/RPG_InventorySystem/Blueprints/BPI_Interactable.Interaction`
  (params (Interactor :type "Actor Object Reference"))
  ;[0 0 0 0.227 22] SERVER: On Interaction
  (`/Engine/EditorBlueprintResources/StandardMacros.IsValid` Interactor
    (:`Is Valid`
      (bind _output_get (set `self.Interactor` Interactor))
      (`self.SetOwner` _output_get)
      (`|ExecutionSequence`
        (:`then_0`
          (switch `int` (`/Game/RPG_InventorySystem/Blueprints/Components/AC_Interactable.Interactable Value` (`self.AC_Interactable`))
            (:`0`
              (`self.Move Forward`))
            (:`1`
              (`self.Move Backward`))))
        (:`then_1`
          (`/Game/RPG_InventorySystem/Blueprints/Components/AC_Interactable.Change Interactable Value` (`self.AC_Interactable`) true)
          (`/Game/RPG_InventorySystem/Blueprints/Components/AC_Interactable.Event Associated Actor Interaction` (`self.AC_Interactable`) (`self.Interactor`)))))))

(event `/Game/RPG_InventorySystem/Blueprints/BPI_Interactable.Initialize`
  ;[0 0 0 0.227 22] On Initialize
  (`/Game/RPG_InventorySystem/Blueprints/Components/AC_Interactable.Setup Interactable References` (`self.AC_Interactable`) (`self.InteractableArea`) (`self.InteractionWidget`) (`|MakeSet` (`self.StaticMesh`) (`self.Lever`) :!type "PrimitiveComponent Object Reference")))

(event `/Game/RPG_InventorySystem/Blueprints/BPI_Interactable.End Interaction`
  (params (Interactor :type "Actor Object Reference"))
  ;[0 0 0 0.227 22] On End Interaction
)

(event `/Game/RPG_InventorySystem/Blueprints/BPI_Interactable.Remove Interaction`
  ;[0 0 0 0.227 22] On Remove Interaction
)

(event `Move Forward`
  ;[1 0.02708 0 0.18] MULTICAST: Move Lever
  (set `/Game/RPG_InventorySystem/Blueprints/Components/AC_Interactable.Timeline Direction` "Forward" (`self.AC_Interactable`))
  (bind (_direction _newtrack_0) (`Timeline|Timeline_0` :!via `PlayFromStart` :!label _label)
    (:`Update`
      (set `self.Lever Location` (`KismetMathLibrary.VLerp` (0.0 0.0 0.0) (0.0 0.0 -28.0) _newtrack_0))
      (set `/Game/RPG_InventorySystem/Blueprints/Components/AC_Interactable.Timeline Position` (`TimelineComponent.GetPlaybackPosition` (`self.Timeline_0`)) (`self.AC_Interactable`)))
    (:`Finished`
      (if (`self.Re-initialize on Moving Finished`)
        (`/Game/RPG_InventorySystem/Blueprints/Components/AC_Interactable.Event Re-initialize` (`self.AC_Interactable`))))))

(event `Move Backward`
  ;[1 0.02708 0 0.18] MULTICAST: Move Lever
  (set `/Game/RPG_InventorySystem/Blueprints/Components/AC_Interactable.Timeline Direction` "Backward" (`self.AC_Interactable`))
  (goto _label :!via `ReverseFromEnd`))

(event `UnPause Timeline`
  (bind _ac_interactable (`self.AC_Interactable`))
  ;[1 0 0.1717 0.264] On UnPause
  (if (`/Game/RPG_InventorySystem/Blueprints/Components/AC_Interactable.Already Interacted` _ac_interactable)
    (switch `ETimelineDirection` (`/Game/RPG_InventorySystem/Blueprints/Components/AC_Interactable.Timeline Direction` _ac_interactable)
      (:`Forward`
        (`self.Move Forward`))
      (:`Backward`
        (`self.Move Backward`)))))

(event `/Game/RPG_InventorySystem/Blueprints/BPI_Interactable.Game Load`
  ;[0 0 0 0.227 22] On Game Load
  (`TimelineComponent.SetPlaybackPosition` (`self.Timeline_0`) (`/Game/RPG_InventorySystem/Blueprints/Components/AC_Interactable.Timeline Position` (`self.AC_Interactable`)) false true)
  (`self.UnPause Timeline`))

(fn `OnRep_Lever Location`
  (`SceneComponent.K2_SetRelativeLocation` (`self.Lever`) (`self.Lever Location`) false false))

(fn `UserConstructionScript`)