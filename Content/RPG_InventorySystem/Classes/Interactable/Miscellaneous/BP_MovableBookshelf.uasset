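; BP_MovableBookshelf is an interactable bookshelf in the RPG inventory system that moves when a player uses its highlightable book.
; Each interaction slides the book via a timeline, then after a short delay calls inherited forward or backward movement, chosen by the interactable component's value.
; The book's location replicates through a RepNotify.
; On game load it restores the timeline position and shows particles if never used.
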(event `self.ReceiveBeginPlay`
  ;[1 0.2073 0 0.488] Begin Play
  (`parent.ReceiveBeginPlay`)
  (set `self.Book Initial Location` (`SceneComponent.RelativeLocation` (`self.InteractableBook`))))

(event `/Game/RPG_InventorySystem/Blueprints/BPI_Interactable.Initialize`
  ;[0 0 0 0.227 22] On Initialize
  (`/Game/RPG_InventorySystem/Blueprints/Components/AC_Interactable.Setup Interactable References` (`self.AC_Interactable`) (`self.InteractableArea`) (`self.InteractionWidget`) (`|MakeSet` (`self.InteractableBook`) :!type "PrimitiveComponent Object Reference")))

(event `/Game/RPG_InventorySystem/Blueprints/BPI_Interactable.Interaction`
  (params (Interactor :type "Actor Object Reference"))
  ;[0 0 0 0.227 22] SERVER: On Interaction
  (`/Engine/EditorBlueprintResources/StandardMacros.IsValid` Interactor
    (:`Is Valid`
      (bind _output_get (set `self.Interactor` Interactor))
      (`self.SetOwner` _output_get)
      (`|ExecutionSequence`
        (:`then_0`
          (switch `int` (`/Game/RPG_InventorySystem/Blueprints/Components/AC_Interactable.Interactable Value` (`self.AC_Interactable`))
            (:`0`
              (`self.Play Book Animation`)
              (`KismetSystemLibrary.Delay` 0.5)
              (`self.Move Forward`)
              (`ActorComponent.Deactivate` (`self.ParticleSystem`)))
            (:`1`
              (`self.Return Book Animation`)
              (`KismetSystemLibrary.Delay` 0.5)
              (`self.Move Backward`))))
        (:`then_1`
          (`/Game/RPG_InventorySystem/Blueprints/Components/AC_Interactable.Change Interactable Value` (`self.AC_Interactable`) true))))))

(event `/Game/RPG_InventorySystem/Blueprints/BPI_Interactable.End Interaction`
  (params (Interactor :type "Actor Object Reference"))
  ;[0 0 0 0.227 22] On End Interaction
)

(event `/Game/RPG_InventorySystem/Blueprints/BPI_Interactable.Remove Interaction`
  ;[0 0 0 0.227 22] On Remove Interaction
)

(event `Play Book Animation`
  (bind _book_initial_location (`self.Book Initial Location`))
  ;[1 0.05908 0 0.426] Play Interactable Book Animation
  (bind (_direction _duration) (`Timeline|Book Location` :!via `PlayFromStart` :!label _label)
    (:`Update`
      (set `self.Book Current Location` (`KismetMathLibrary.VLerp` _book_initial_location (+ _book_initial_location (0.0 6.0 0.0)) _duration)))))

(event `Return Book Animation`
  ;[1 0.05908 0 0.426] Play Interactable Book Animation
  (goto _label :!via `ReverseFromEnd`))

(event `/Game/RPG_InventorySystem/Blueprints/BPI_Interactable.Game Load`
  ;[0 0 0 0.227 22] On Game Load
  (`self.Set Timeline Postion` (`/Game/RPG_InventorySystem/Blueprints/Components/AC_Interactable.Timeline Position` (`self.AC_Interactable`)))
  (if (not (`/Game/RPG_InventorySystem/Blueprints/Components/AC_Interactable.Already Interacted` (`self.AC_Interactable`)))
    (`ActorComponent.Activate` (`self.ParticleSystem`) true)))

(fn `OnRep_Book Current Location`
  (`SceneComponent.K2_SetRelativeLocation` (`self.InteractableBook`) (`self.Book Current Location`) false false))

(fn `Update Travel Transform`
  (params (`Current Time` :type "Float (double-precision)"))
  (`parent.Update Travel Transform` `Current Time`))

(fn `UserConstructionScript`
  (`parent.UserConstructionScript`))