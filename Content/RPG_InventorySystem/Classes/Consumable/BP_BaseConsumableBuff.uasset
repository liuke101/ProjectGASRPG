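; Base actor for a consumable buff in the RPG inventory system, applying a stat change to its owner on BeginPlay and destroying itself when finished.
; Effect selects an instant add, repeated timer ticks (Health and Stamina only) or a temporary, resettable add, applied through server calls on the stats component.
; A rate-scaled timeline feeds progress to the owner's buffs component for a circular animation.
; Optional Drunk or Night Vision effects add post-process components, removed on expiry.
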(event `Play Additional Effect`
  ;[0.5489 0 1 0.41] Additional Effects
  (switch `/Game/RPG_InventorySystem/ItemsData/Enums/E_AdditionalBuffEffect` (`self.Additional Effect`)
    (:`NewEnumerator0`
      (`/Engine/EditorBlueprintResources/StandardMacros.IsValid` (`self.PostProcess Drunk`)
        (:`Is Not Valid`
          (bind _returnvalue (`AddComponent|NODE_AddPostProcessComponent-0`))
          (set `self.PostProcess Drunk` _returnvalue))))
    (:`NewEnumerator1`
      (`/Engine/EditorBlueprintResources/StandardMacros.IsValid` (`self.PostProcess NightVision`)
        (:`Is Not Valid`
          (bind _returnvalue_2 (`AddComponent|NODE_AddPostProcessComponent-3`))
          (set `self.PostProcess NightVision` _returnvalue_2))))))

(event `Remove Additional Effect`
  (bind _postprocess_nightvision (`self.PostProcess NightVision`))
  (bind _postprocess_drunk (`self.PostProcess Drunk`))
  ;[0.5489 0 1 0.41] Additional Effects
  (switch `/Game/RPG_InventorySystem/ItemsData/Enums/E_AdditionalBuffEffect` (`self.Additional Effect`)
    (:`NewEnumerator0`
      (`/Engine/EditorBlueprintResources/StandardMacros.IsValid` _postprocess_drunk
        (:`Is Valid`
          (`ActorComponent.K2_DestroyComponent` _postprocess_drunk))))
    (:`NewEnumerator1`
      (`/Engine/EditorBlueprintResources/StandardMacros.IsValid` _postprocess_nightvision
        (:`Is Valid`
          (`ActorComponent.K2_DestroyComponent` _postprocess_nightvision))))))

(event `self.ReceiveBeginPlay`
  ;[1 0 0.01425 0.551] On Begin Play
  (bind _returnvalue (`/Game/RPG_InventorySystem/Blueprints/BFL_Inventory.Get AC Stats` (`self.GetOwner`)))
  (set `self.Stats Component` _returnvalue)
  (bind _returnvalue_2 (`/Game/RPG_InventorySystem/Blueprints/BFL_Inventory.Get AC Consumable Buffs` (`self.GetOwner`)))
  (set `self.Consumable Buffs Component` _returnvalue_2)
  (`self.On Use`)
  (`self.Play Additional Effect`)
  (`GameplayStatics.PlaySound2D` (`self.Consum Sound`) 1.0 1.0 0.0 null null))

(event `Event Remove Value from Stat`
  ;[1 0 0.06404 0.567] Remove Value
  (`/Game/RPG_InventorySystem/Blueprints/Components/AC_Stats.Server Remove Stat Value` (`self.Stats Component`) (`self.Stat`) (`self.Value`)))

(event `On Use`
  ;[0.007438 1 0 0.509] On Use
  (switch `/Game/RPG_InventorySystem/ItemsData/Enums/E_BuffEffectCategory` (`self.Effect`)
    (:`NewEnumerator1`
      (`self.Event Add Value to Stat`)
      (`self.On Remove`))
    (:`NewEnumerator2`
      (`self.Event Add Value over Duration`)
      (`self. Initialize Timeline Animation`))
    (:`NewEnumerator3`
      (`self.Event Add Value for Duration`)
      (`self. Initialize Timeline Animation`))))

(event `On Remove`
  ;[0.007438 1 0 0.509] On Remove
  (switch `/Game/RPG_InventorySystem/ItemsData/Enums/E_BuffEffectCategory` (`self.Effect`)
    (:`NewEnumerator0`
      _)
    (:`NewEnumerator1`
      _)
    (:`NewEnumerator2`
      (`KismetSystemLibrary.K2_ClearAndInvalidateTimerHandle` (`self.Over Duration Timer`)))
    (:`NewEnumerator3`
      (`self.Event Remove Value from Stat`)
      (`KismetSystemLibrary.K2_ClearAndInvalidateTimerHandle` (`self.For Duration Timer`))))
  (`self.Remove Additional Effect`)
  (`self.K2_DestroyActor`))

(event `Event Add Value to Stat`
  ;[1 0 0.06404 0.567] Add Value
  (`/Game/RPG_InventorySystem/Blueprints/Components/AC_Stats.Server Add Stat Value` (`self.Stats Component`) (`self.Stat`) (`self.Value`)))

(event `Initialize Timeline Animation`
  ;[1 0.391 0 0.509] Initialize Timeline
  (`/Game/RPG_InventorySystem/Blueprints/Components/AC_ConsumableBuffs.Event Initialize Circular Animation` (`self.Consumable Buffs Component`) (`self.Stat`))
  (`TimelineComponent.SetPlayRate` (`self.Effect Timeline`) (`KismetMathLibrary.SafeDivide` 1.0 (- (`self.Duration`) (`KismetMathLibrary.SafeDivide` (`self.Duration`) (`KismetMathLibrary.Conv_IntToDouble` (`self.Number of Reps`))))))
  (bind (_direction _value) (`Timeline|Effect Timeline` :!via `PlayFromStart`)
    (:`Update`
      (`BlueprintMapLibrary.Map_Add` (`/Game/RPG_InventorySystem/Blueprints/Components/AC_ConsumableBuffs.Stats Decimal` (`self.Consumable Buffs Component`)) (`self.Stat`) _value))))

(event `Event Add Value over Duration`
  ;[1 0.05473 0 0.473] Over Duration
  (if (not (`KismetSystemLibrary.K2_TimerExistsHandle` (`self.Over Duration Timer`)))
    (bind _returnvalue (`KismetSystemLibrary.K2_SetTimerDelegate` (delegate `Event Add Value over Duration`) (`KismetMathLibrary.SafeDivide` (`self.Duration`) (`KismetMathLibrary.Conv_IntToDouble` (`self.Number of Reps`))) true))
    (set `self.Over Duration Timer` _returnvalue))
  (switch `/Game/RPG_InventorySystem/ItemsData/Enums/E_StatCategory` (`self.Stat`)
    (:`NewEnumerator0`
      _)
    (:`NewEnumerator1`
      _))
  (`self.Event Add Value to Stat`)
  (bind _result (`/Engine/EditorBlueprintResources/StandardMacros.IncrementInt` (`self.Current Rep`))
    (:`  `
      (if (<= (`self.Number of Reps`) _result)
        (`self.On Remove`)))))

(event `Event Add Value for Duration`
  ;[1 0.06501 0 0.499] For Duration
  (if (not (`KismetSystemLibrary.K2_TimerExistsHandle` (`self.For Duration Timer`)))
    (bind _returnvalue (`KismetSystemLibrary.K2_SetTimerDelegate` (delegate `Event Add Value for Duration`) (`self.Duration`)))
    (set `self.For Duration Timer` _returnvalue)
    (`self.Event Add Value to Stat`)
    (else
      (`self.On Remove`))))

(event `Reset Add Value for Duration`
  ;[1 0.179 0 0.567] Reset For Duration
  (switch `/Game/RPG_InventorySystem/ItemsData/Enums/E_BuffEffectCategory` (`self.Effect`)
    (:`NewEnumerator3`
      (if (`KismetSystemLibrary.K2_TimerExistsHandle` (`self.For Duration Timer`))
        (`KismetSystemLibrary.K2_ClearAndInvalidateTimerHandle` (`self.For Duration Timer`))
        (`self.Event Remove Value from Stat`)
        (`self.Event Add Value for Duration`)))))

(fn `UserConstructionScript`)