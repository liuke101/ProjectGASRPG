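; BP_PlayerCapture is a stand-in character filmed by a SceneCaptureComponent2D to show the player's equipped items in the RPG inventory system.
; PlayerEquipment attach and detach dispatchers drive it: armor swaps leader-posed skeletal meshes, while weapons and shields spawn as socketed actors.
; The capture's show-only list limits it to this actor and spawned gear.
; Per-frame capture runs only between StartCapture and EndCapture, alongside a temporary wind source.
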(event `Event Start Capture`
  ;[0 1 0.08226 0.227] Start Capture
  (set `SceneCaptureComponent.bCaptureEveryFrame` true (`self.SceneCaptureComponent2D`))
  (`self.Spawn Wind Component` 1.0 0.5))

(event `Event End Capture`
  (bind _wind (`self.Wind`))
  (bind _skeletalmesh (`self.SkeletalMesh`))
  ;[1 0 0.01016 0.269] End Capture
  (set `SceneCaptureComponent.bCaptureEveryFrame` false (`self.SceneCaptureComponent2D`))
  (`/Engine/EditorBlueprintResources/StandardMacros.IsValid` _wind
    (:`Is Valid`
      (`self.K2_DestroyActor` _wind)
      (`SceneComponent.K2_SetRelativeRotation` _skeletalmesh (`KismetMathLibrary.MakeRotator` (.roll (`SceneComponent.RelativeRotation` _skeletalmesh)) (.pitch (`SceneComponent.RelativeRotation` _skeletalmesh))) false false))))

(event `Initialize Player Capture`
  (params (`Player Equipment` :type "/Game/RPG_InventorySystem/Blueprints/Components/AC_PlayerEquipment Object Reference"))
  ;[0 0.3476 1 0.217] Set References
  (`/Engine/EditorBlueprintResources/StandardMacros.IsValid` `Player Equipment`
    (:`Is Valid`
      (set `self.Player Equipment` `Player Equipment`)
      (`/Engine/EditorBlueprintResources/StandardMacros.IsValid` (`self.Player Equipment`)
        (:`Is Valid`
          (add `/Game/RPG_InventorySystem/Blueprints/Components/AC_PlayerEquipment.On Item Attach` (`self.Player Equipment`) (`|CreateDelegate` :!event `Attach Item`))
          (add `/Game/RPG_InventorySystem/Blueprints/Components/AC_PlayerEquipment.On Item Detach` (`self.Player Equipment`) (`|CreateDelegate` :!event `Detach Item`)))))))

(fn `Attach Item`
  (params (`Item Data` :type "/Game/RPG_InventorySystem/ItemsData/Structs/Item/S_ItemData Structure"))
  (locals (`L Item Slot` :type "/Game/RPG_InventorySystem/ItemsData/Enums/E_ItemSlot Enum") (`L Equippable Item` :type "/Game/RPG_InventorySystem/Classes/Equippable/BP_BaseEquippable Class Reference") (`L Skeletal` :type "SkeletalMesh Object Reference") (`L Weapon Type` :type "/Game/RPG_InventorySystem/ItemsData/Enums/E_WeaponType Enum"))
  (bind ((`EquipmentSlot_82_D8E166834B91EEF8631726AE76BDFFE0` _equipmentslot) (`Class_81_28B5086542C7943CC83294BF5B57815A` _class)) (break `/Game/RPG_InventorySystem/ItemsData/Structs/Item/S_ItemData` `Item Data`))
  (bind _equipped_shield_slot (`self.Equipped Shield Slot`))
  (bind _equipped_weapon_slot (`self.Equipped Weapon Slot`))
  (bind (_weapon_type _weapon_subtype _equippable_class _skeletal_mesh) (defaults `Object` _class))
  (bind _returnvalue (select `/Game/RPG_InventorySystem/ItemsData/Enums/E_ItemSlot` (`local.L Item Slot`) :`NewEnumerator1` (`self.Head`) :`NewEnumerator2` (`self.Gloves`) :`NewEnumerator4` (`self.Chest`) :`NewEnumerator5` (`self.Legs`) :`NewEnumerator6` (`self.Boots`) :!type "SkinnedMeshComponent Object Reference"))
  (`/Game/RPG_InventorySystem/Blueprints/BML_Inventory.Is Item Class Valid?` `Item Data`
    (:`Valid`
      (set `local.L Item Slot` _equipmentslot)
      (set `local.L Weapon Type` _weapon_type)
      (set `local.L Equippable Item` _equippable_class)
      (set `local.L Skeletal` _skeletal_mesh)
      (switch `/Game/RPG_InventorySystem/ItemsData/Enums/E_ItemSlot` (`local.L Item Slot`)
        (:`NewEnumerator1`
          ;[0.05725 1 0 0.285 22] Attach Armor [Skeletal]
          (`/Engine/EditorBlueprintResources/StandardMacros.IsValid` _returnvalue :!label _label
            (:`Is Valid`
              (`SkinnedMeshComponent.SetSkinnedAssetAndUpdate` _returnvalue (`local.L Skeletal`) true)
              (`SkinnedMeshComponent.SetLeaderPoseComponent` _returnvalue (`self.SkeletalMesh`) true false))))
        (:`NewEnumerator2`
          (goto _label))
        (:`NewEnumerator4`
          (goto _label))
        (:`NewEnumerator5`
          (goto _label))
        (:`NewEnumerator6`
          (goto _label))
        (:`NewEnumerator7`
          ;[1 0.5216 0 0.243 22] Attach Weapon [Actor Class Ref]
          (`/Engine/EditorBlueprintResources/StandardMacros.IsValid` _equipped_weapon_slot
            (:`Is Valid`
              (`self.K2_DestroyActor` _equipped_weapon_slot))
            (:`Is Not Valid`
              _))
          (bind _returnvalue_2 (`|SpawnActorFromClass` (`local.L Equippable Item`) (`self.GetTransform`) "Undefined" "SelectDefaultAtRuntime" null null))
          (set `self.Equipped Weapon Slot` _returnvalue_2)
          (`SceneCaptureComponent.ShowOnlyActorComponents` (`self.SceneCaptureComponent2D`) (`self.Equipped Weapon Slot`) true)
          (`self.K2_AttachToComponent` (`self.Equipped Weapon Slot`) (`self.SkeletalMesh`) (select `/Game/RPG_InventorySystem/ItemsData/Enums/E_WeaponType` (`local.L Weapon Type`) :`NewEnumerator3` "main_hand" :`NewEnumerator0` "main_hand" :`NewEnumerator1` "two_hand" :`NewEnumerator2` "main_hand" :!type "Name") "SnapToTarget" "SnapToTarget" "SnapToTarget" false))
        (:`NewEnumerator12`
          ;[1 0.02652 0 0.243 22] Attach Shield [Actor Class Ref]
          (`/Engine/EditorBlueprintResources/StandardMacros.IsValid` _equipped_shield_slot
            (:`Is Valid`
              (`self.K2_DestroyActor` _equipped_shield_slot))
            (:`Is Not Valid`
              _))
          (bind _returnvalue_3 (`|SpawnActorFromClass` (`local.L Equippable Item`) (`self.GetTransform`) "Undefined" "SelectDefaultAtRuntime" null null))
          (set `self.Equipped Shield Slot` _returnvalue_3)
          (`SceneCaptureComponent.ShowOnlyActorComponents` (`self.SceneCaptureComponent2D`) (`self.Equipped Shield Slot`) true)
          (`self.K2_AttachToComponent` (`self.Equipped Shield Slot`) (`self.SkeletalMesh`) (select `/Game/RPG_InventorySystem/ItemsData/Enums/E_WeaponType` (`local.L Weapon Type`) :`NewEnumerator3` "shield" :`NewEnumerator0` "off_hand" :`NewEnumerator1` "two_hand" :`NewEnumerator2` "shield" :!type "Name") "SnapToTarget" "SnapToTarget" "SnapToTarget" false))))))

(fn `Detach Item`
  (params (`Item Data` :type "/Game/RPG_InventorySystem/ItemsData/Structs/Item/S_ItemData Structure"))
  (locals (`L Item Slot` :type "/Game/RPG_InventorySystem/ItemsData/Enums/E_ItemSlot Enum"))
  (bind _equipped_shield_slot (`self.Equipped Shield Slot`))
  (bind _equipped_weapon_slot (`self.Equipped Weapon Slot`))
  (bind _output_get (set `local.L Item Slot` (`.EquipmentSlot_82_D8E166834B91EEF8631726AE76BDFFE0` (break `/Game/RPG_InventorySystem/ItemsData/Structs/Item/S_ItemData` `Item Data`))))
  (switch `/Game/RPG_InventorySystem/ItemsData/Enums/E_ItemSlot` _output_get
    (:`NewEnumerator1`
      ;[0.05725 1 0 0.285 22] Detach Armor [Skeletal]
      (`SkinnedMeshComponent.SetSkinnedAssetAndUpdate` (`self.Head`) null true))
    (:`NewEnumerator2`
      (`SkinnedMeshComponent.SetSkinnedAssetAndUpdate` (`self.Gloves`) null true))
    (:`NewEnumerator4`
      (`SkinnedMeshComponent.SetSkinnedAssetAndUpdate` (`self.Chest`) null true))
    (:`NewEnumerator5`
      (`SkinnedMeshComponent.SetSkinnedAssetAndUpdate` (`self.Legs`) null true))
    (:`NewEnumerator6`
      (`SkinnedMeshComponent.SetSkinnedAssetAndUpdate` (`self.Boots`) null true))
    (:`NewEnumerator7`
      ;[1 0.5216 0 0.243 22] Detach Weapon [Static]
      (`/Engine/EditorBlueprintResources/StandardMacros.IsValid` _equipped_weapon_slot
        (:`Is Valid`
          (`self.K2_DestroyActor` _equipped_weapon_slot))))
    (:`NewEnumerator12`
      ;[1 0.02652 0 0.243 22] Detach Shield [Static]
      (`/Engine/EditorBlueprintResources/StandardMacros.IsValid` _equipped_shield_slot
        (:`Is Valid`
          (`self.K2_DestroyActor` _equipped_shield_slot))))))

(fn `Spawn Wind Component`
  (params (Strength :type "Float (double-precision)" :default 1.0) (Speed :type "Float (double-precision)" :default 1.0))
  (bind _returnvalue (`|SpawnActorFromClass` "/Script/Engine.WindDirectionalSource" (`SceneComponent.GetRelativeTransform` (`self.Wind Position`)) "AlwaysSpawn" "MultiplyWithRoot" null null))
  (bind _output_get (set `self.Wind` _returnvalue))
  (bind _component (`WindDirectionalSource.Component` _output_get))
  (`WindDirectionalSourceComponent.SetStrength` _component (`local.Strength`))
  (`WindDirectionalSourceComponent.SetSpeed` _component (`local.Speed`)))

(fn `UserConstructionScript`
  (`SceneCaptureComponent.ShowOnlyActorComponents` (`self.SceneCaptureComponent2D`) self true))