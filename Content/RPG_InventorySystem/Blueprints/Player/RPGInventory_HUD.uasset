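; HUD actor for the RPG inventory system that owns the player's main HUD widget.
; On BeginPlay it creates WB_HUD for the owning controller, adding it to the player screen when several local players exist, otherwise to the viewport.
; ShowLootBar and HideLootBar events forward loot bar toggles to that widget when it is valid.
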(event `self.ReceiveBeginPlay`
  (bind _hud_ref (`self.HUD Ref`))
  ;[1 0 0.0296 0.53] On Begin Play
  (bind _returnvalue (`|CreateWidget` "/Game/RPG_InventorySystem/UI/HUD/WB_HUD.WB_HUD_C" (`self.GetOwningPlayerController`)))
  (set `self.HUD Ref` _returnvalue)
  (if (`KismetSystemLibrary.HasMultipleLocalPlayers`)
    (`UserWidget.AddToPlayerScreen` _hud_ref 0)
    (else
      (`UserWidget.AddToViewport` _hud_ref 0))))

(event `Show LootBar`
  (bind _hud_ref (`self.HUD Ref`))
  ;[0 0.8314 1 0.452] Toggle LootBar
  (`/Engine/EditorBlueprintResources/StandardMacros.IsValid` _hud_ref
    (:`Is Valid`
      (`/Game/RPG_InventorySystem/UI/HUD/WB_HUD.Show LootBar` _hud_ref))))

(event `Hide LootBar`
  (bind _hud_ref (`self.HUD Ref`))
  ;[0 0.8314 1 0.452] Toggle LootBar
  (`/Engine/EditorBlueprintResources/StandardMacros.IsValid` _hud_ref
    (:`Is Valid`
      (`/Game/RPG_InventorySystem/UI/HUD/WB_HUD.Hide LootBar` _hud_ref))))

(fn `UserConstructionScript`)