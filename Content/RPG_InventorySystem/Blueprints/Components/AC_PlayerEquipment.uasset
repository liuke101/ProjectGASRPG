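; Player controller component that manages a character's equipment as a slot-to-item map for armor, weapon, shield and pocket slots.
; Builds starting gear from data table rows and handles equipping, stacking, swapping and removal, with level checks and one-hand, two-hand and off-hand rules.
; Changes run on the server and reach the owning client through RPCs and dispatchers.
; Armor updates character meshes, while weapons and shields spawn as socket-attached actors.
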(fn `Add Item to Equipment Array`
  (params (`Item Data` :type "/Game/RPG_InventorySystem/ItemsData/Structs/Item/S_ItemData Structure (by ref)") (`Equipment Slot` :type "/Game/RPG_InventorySystem/ItemsData/Enums/E_ItemSlot Enum" :default "NewEnumerator0"))
  ;[1 0 0.06858 0.493] SERVER: Add Item to Equipment Data
  (`/Game/RPG_InventorySystem/Blueprints/BML_Inventory.Switch Has Owner Authority`
    (:`Authority`
      (bind _structout (setmembers `/Game/RPG_InventorySystem/ItemsData/Structs/Item/S_ItemData` :`StructRef` `Item Data` :`Equipment Slot` `Equipment Slot` :`Is Equipped` true))
      (`BlueprintMapLibrary.Map_Add` (`self.Equipment Data`) `Equipment Slot` _structout)
      ;[1 0.9656 0 0.493] IF STANDALONE: Call Event Dispatcher
      (if (`KismetSystemLibrary.IsStandalone`)
        (`self.On Added to Equipment` (`local.Item Data`))
        (else
          ;[0.1707 1 0 0.493] CLIENT: Update Item
          (`self.Client Update Added Item` (`local.Item Data`)))))))

(fn `Add to Stack in Equipment`
  (params (`Item Data` :type "/Game/RPG_InventorySystem/ItemsData/Structs/Item/S_ItemData Structure") (`Equipment Slot` :type "/Game/RPG_InventorySystem/ItemsData/Enums/E_ItemSlot Enum" :default "NewEnumerator0"))
  (bind (_value _returnvalue) (`BlueprintMapLibrary.Map_Find` (`self.Equipment Data`) `Equipment Slot`))
  (if _returnvalue
    (bind _structout (setmembers `/Game/RPG_InventorySystem/ItemsData/Structs/Item/S_ItemData` :`StructRef` _value :`Quantity` (+ (`.Quantity_76_AD4B883E4427C3E60B4B22B072F4E7C9` (break `/Game/RPG_InventorySystem/ItemsData/Structs/Item/S_ItemData` _value)) (`.Quantity_76_AD4B883E4427C3E60B4B22B072F4E7C9` (break `/Game/RPG_InventorySystem/ItemsData/Structs/Item/S_ItemData` (`local.Item Data`))))))
    (`self.Add Item to Equipment Array` _structout (`.EquipmentSlot_82_D8E166834B91EEF8631726AE76BDFFE0` (break `/Game/RPG_InventorySystem/ItemsData/Structs/Item/S_ItemData` _structout)))))

(fn `Assign Item from Equipment Slot`
  (params (`Item Data` :type "/Game/RPG_InventorySystem/ItemsData/Structs/Item/S_ItemData Structure"))
  (returns (`In Slot Data` :type "/Game/RPG_InventorySystem/ItemsData/Structs/Item/S_ItemData Structure"))
  (if (`BlueprintSetLibrary.Set_Contains` (`|MakeSet` "NewEnumerator8" "NewEnumerator9" "NewEnumerator10" "NewEnumerator11" :!type "/Game/RPG_InventorySystem/ItemsData/Enums/E_ItemSlot Enum") (`.EquipmentSlot_82_D8E166834B91EEF8631726AE76BDFFE0` (break `/Game/RPG_InventorySystem/ItemsData/Structs/Item/S_ItemData` (`local.Item Data`))))
    ;[1 0.7046 0 0.358] Assign Item from Empty/Default Slot [Consumables]
    (bind _slot (`/Game/RPG_InventorySystem/Blueprints/BML_Inventory.Find Empty Equipment Slot` (`self.Equipment Data`) (`|MakeArray` "NewEnumerator8" "NewEnumerator9" "NewEnumerator10" "NewEnumerator11" :!type "/Game/RPG_InventorySystem/ItemsData/Enums/E_ItemSlot Enum") "NewEnumerator8")
      (:`Found`
        _)
      (:`Not Found`
        _))
    (return (`.Item Data` (`self.Get Item by Equipment Slot` _slot)))
    (else
      ;[1 0.03104 0 0.608] #Check if Item is a One-Hand [AND Off-Hand is Enabled]
      (if (and (`self.Enable Off-Hand`) (`|EnumEquality` (defaults `Object` (`.Class_81_28B5086542C7943CC83294BF5B57815A` (break `/Game/RPG_InventorySystem/ItemsData/Structs/Item/S_ItemData` (`local.Item Data`)))) "NewEnumerator0"))
        ;[1 0.03104 0 0.608] #Check if there is already One-Hand Weapon in [Shield]Slot
        (if (not (`self.Get Item by Equipment Slot` "NewEnumerator12"))
          ;[1 0.7046 0 0.358] Assign Item from Empty/Default Slot [One-hand]
          (bind _slot_2 (`/Game/RPG_InventorySystem/Blueprints/BML_Inventory.Find Empty Equipment Slot` (`self.Equipment Data`) (`|MakeArray` "NewEnumerator7" "NewEnumerator12" :!type "/Game/RPG_InventorySystem/ItemsData/Enums/E_ItemSlot Enum") "NewEnumerator7")
            (:`Found`
              _)
            (:`Not Found`
              _))
          (return (`.Item Data` (`self.Get Item by Equipment Slot` _slot_2)))
          (else
            ;[0.1261 0 1 0.577] Assign Item from Weapon Slot
            (return (`.Item Data` (`self.Get Item by Equipment Slot` "NewEnumerator7")))))
        (else
          ;[0.1352 1 0 0.379] Assign Item from equal Slot [Default]
          (return (`.Item Data` (`self.Get Item by Equipment Slot` (`.EquipmentSlot_82_D8E166834B91EEF8631726AE76BDFFE0` (break `/Game/RPG_InventorySystem/ItemsData/Structs/Item/S_ItemData` (`local.Item Data`)))))))))))

(fn `Attach Equipped Item to Socket`
  (params (Slot :type "/Game/RPG_InventorySystem/ItemsData/Enums/E_ItemSlot Enum" :default "NewEnumerator0") (`Socket Name` :type Name))
  (bind _returnvalue (`self.Get Equipped Actor Reference` Slot))
  (`/Engine/EditorBlueprintResources/StandardMacros.IsValid` _returnvalue
    (:`Is Valid`
      (`Actor.K2_AttachToComponent` _returnvalue (`Character.Mesh` (`self.Owning Character`)) (`local.Socket Name`) "SnapToTarget" "SnapToTarget" "SnapToTarget" false))))

(fn `Attach Item to Equipment`
  (params (`Item Data` :type "/Game/RPG_InventorySystem/ItemsData/Structs/Item/S_ItemData Structure"))
  (locals (`L Item Slot` :type "/Game/RPG_InventorySystem/ItemsData/Enums/E_ItemSlot Enum") (`L Skeletal` :type "SkeletalMesh Object Reference"))
  (bind ((`EquipmentSlot_82_D8E166834B91EEF8631726AE76BDFFE0` _equipmentslot) (`Class_81_28B5086542C7943CC83294BF5B57815A` _class)) (break `/Game/RPG_InventorySystem/ItemsData/Structs/Item/S_ItemData` `Item Data`))
  (`/Game/RPG_InventorySystem/Blueprints/BML_Inventory.Is Item Class Valid?` `Item Data`
    (:`Valid`
      (set `local.L Item Slot` _equipmentslot)
      (set `local.L Skeletal` (defaults `Object` _class))
      (`/Engine/EditorBlueprintResources/StandardMacros.IsValid` (`self.Owning Character`)
        (:`Is Valid`
          (`self.On Item Attach` (`local.Item Data`))
          (switch `/Game/RPG_InventorySystem/ItemsData/Enums/E_ItemSlot` (`local.L Item Slot`)
            (:`NewEnumerator1`
              ;[0.05725 1 0 0.285 22] Attach to Master Pose
              (`/Game/RPG_InventorySystem/Blueprints/Player/BP_RPGInventoryCharacter.Server Update Equipment Mesh` (`self.Owning Character`) (`local.L Item Slot`) (`local.L Skeletal`) :!label _label) ; Called on Server inside RPGInventoryCharacterBP
            )
            (:`NewEnumerator2`
              (goto _label))
            (:`NewEnumerator3`
              (goto _label))
            (:`NewEnumerator4`
              (goto _label))
            (:`NewEnumerator5`
              (goto _label))
            (:`NewEnumerator6`
              (goto _label))
            (:`NewEnumerator7`
              ;[1 0.8208 0 0.285 22] Attach to Socket
              (`self.Server Spawn Equippable Actor` (`local.Item Data`) (`self.Owning Character`) :!label _label_2))
            (:`NewEnumerator12`
              (goto _label_2))))))))

(fn `Build Equipment`
  (locals (`L Empty Data` :type "/Game/RPG_InventorySystem/ItemsData/Structs/Item/S_ItemData Structure"))
  (bind _enumvalue (foreach `/Game/RPG_InventorySystem/ItemsData/Enums/E_ItemSlot` false)
    (:`LoopBody`
      (bind (_value _returnvalue) (`BlueprintMapLibrary.Map_Find` (`self.Equipment Data`) _enumvalue))
      (if _returnvalue
        (bind _structout (setmembers `/Game/RPG_InventorySystem/ItemsData/Structs/Item/S_ItemData` :`StructRef` _value :`Equipment Slot` _enumvalue :`Is Equipped` true))
        (`BlueprintMapLibrary.Map_Add` (`self.Equipment Data`) _enumvalue _structout)
        (else
          (bind _structout_2 (setmembers `/Game/RPG_InventorySystem/ItemsData/Structs/Item/S_ItemData` :`StructRef` (`local.L Empty Data`) :`Equipment Slot` _enumvalue))
          (`BlueprintMapLibrary.Map_Add` (`self.Equipment Data`) _enumvalue _structout_2))))))

(fn `Build Initial Equipment`
  (locals (`L Item Data` :type "/Game/RPG_InventorySystem/ItemsData/Structs/Item/S_ItemData Structure"))
  (bind _returnvalue (`Actor.GetComponentByClass` (`self.GetOwner`) "/Game/RPG_InventorySystem/Blueprints/Components/AC_InventoryCore.AC_InventoryCore_C"))
  (for _array_element (`self.Initial Equipment`)
    (bind (_datatable _rowname) (break `DataTableRowHandle` (break `/Game/RPG_InventorySystem/ItemsData/Structs/Item/S_SingleDTItem` _array_element)))
    ;[1 0.163 0 0.138 37] Add single row to Equipment Data
    (bind _returnvalue_2 (`|GetDataTableRow` _datatable _rowname)
      (:`then`
        (bind _structout (setmembers `/Game/RPG_InventorySystem/ItemsData/Structs/Item/S_ItemData` :`StructRef` _returnvalue_2 :`Quantity` (`KismetMathLibrary.Clamp` (`.Quantity_5_301361FE450B4BCA98AFAF9972720D7A` (break `/Game/RPG_InventorySystem/ItemsData/Structs/Item/S_SingleDTItem` _array_element)) 1 (`.Quantity_5_301361FE450B4BCA98AFAF9972720D7A` (break `/Game/RPG_InventorySystem/ItemsData/Structs/Item/S_SingleDTItem` _array_element)))))
        (bind _output_get (set `local.L Item Data` _structout))
        (bind _in_slot_data (`self.Assign Item from Equipment Slot` _output_get))
        (`self.Add Item to Equipment Array` (`local.L Item Data`) (`.EquipmentSlot_82_D8E166834B91EEF8631726AE76BDFFE0` (break `/Game/RPG_InventorySystem/ItemsData/Structs/Item/S_ItemData` _in_slot_data)))
        (`self.Attach Item to Equipment` (`local.L Item Data`))
        (`/Engine/EditorBlueprintResources/StandardMacros.IsValid` _returnvalue
          (:`Is Valid`
            (`/Game/RPG_InventorySystem/Blueprints/Components/AC_InventoryCore.Add Weight to Inventory` _returnvalue (`/Game/RPG_InventorySystem/Blueprints/BML_Inventory.Calculate Stacked Item Weight` (`local.L Item Data`))))))))
  ;[0.8225 1 0 0.18] Clear Data Table Variables on Completed
  (`KismetArrayLibrary.Array_Clear` (`self.Initial Equipment`)))

(fn `Can Item be Equipped?`
  (params (`Item Data` :type "/Game/RPG_InventorySystem/ItemsData/Structs/Item/S_ItemData Structure"))
  (returns (`Return Value` :type Boolean) (`Failure Message` :type Text))
  (bind _returnvalue (`Actor.GetComponentByClass` (`self.GetOwner`) "/Game/RPG_InventorySystem/Blueprints/Components/AC_Leveling.AC_Leveling_C"))
  (if (and (`KismetSystemLibrary.IsValid` _returnvalue) (select `bool` (`self.Check Required Item Level`) :`false` true :`true` (>= (`/Game/RPG_InventorySystem/Blueprints/Components/AC_Leveling.Current Level` _returnvalue) (defaults `Object` (`.Class_81_28B5086542C7943CC83294BF5B57815A` (break `/Game/RPG_InventorySystem/ItemsData/Structs/Item/S_ItemData` (`local.Item Data`)))))))
    (return true "")
    (else
      (return false "Higher level required."))))

(fn `Destroy Equippable Actor`
  (params (Slot :type "/Game/RPG_InventorySystem/ItemsData/Structs/Item/S_ItemData Structure"))
  (bind _returnvalue (select `/Game/RPG_InventorySystem/ItemsData/Enums/E_ItemSlot` (`.EquipmentSlot_82_D8E166834B91EEF8631726AE76BDFFE0` (break `/Game/RPG_InventorySystem/ItemsData/Structs/Item/S_ItemData` Slot)) :`NewEnumerator7` (`self.Equipped Weapon Slot`) :`NewEnumerator12` (`self.Equipped Shield Slot`)))
  ;[1 0 0.02348 0.478] SERVER: Destroy Equippable Actor
  (`/Game/RPG_InventorySystem/Blueprints/BML_Inventory.Switch Has Owner Authority`
    (:`Authority`
      (`/Engine/EditorBlueprintResources/StandardMacros.IsValid` _returnvalue
        (:`Is Valid`
          (`Actor.K2_DestroyActor` _returnvalue))))))

(fn `Detach Item from Equipment`
  (params (`Item Data` :type "/Game/RPG_InventorySystem/ItemsData/Structs/Item/S_ItemData Structure"))
  (locals (`L Item Slot` :type "/Game/RPG_InventorySystem/ItemsData/Enums/E_ItemSlot Enum"))
  (bind _item_data (`local.Item Data`))
  (`/Engine/EditorBlueprintResources/StandardMacros.IsValid` (`self.Owning Character`)
    (:`Is Valid`
      (`self.On Item Detach` _item_data)
      (bind _output_get (set `local.L Item Slot` (`.EquipmentSlot_82_D8E166834B91EEF8631726AE76BDFFE0` (break `/Game/RPG_InventorySystem/ItemsData/Structs/Item/S_ItemData` _item_data))))
      (switch `/Game/RPG_InventorySystem/ItemsData/Enums/E_ItemSlot` _output_get
        (:`NewEnumerator1`
          ;[0.05725 1 0 0.285 22] Detach Armor
          (`/Game/RPG_InventorySystem/Blueprints/Player/BP_RPGInventoryCharacter.Server Update Equipment Mesh` (`self.Owning Character`) (`local.L Item Slot`) null :!label _label))
        (:`NewEnumerator2`
          (goto _label))
        (:`NewEnumerator3`
          (goto _label))
        (:`NewEnumerator4`
          (goto _label))
        (:`NewEnumerator5`
          (goto _label))
        (:`NewEnumerator6`
          (goto _label))
        (:`NewEnumerator7`
          ;[1 0.5216 0 0.243 22] Detach Weapon Slot
          (`self.Server Destroy Equippable Actor` (`local.Item Data`) :!label _label_2))
        (:`NewEnumerator12`
          (goto _label_2))))))

(fn `Get Equipment Items`
  (returns (Items :type "Array of /Game/RPG_InventorySystem/ItemsData/Structs/Item/S_ItemData Structure"))
  (bind _values (`BlueprintMapLibrary.Map_Values` (`self.Equipment Data`)))
  (return _values))

(fn `Get Equipped Actor Reference`
  (params (Slot :type "/Game/RPG_InventorySystem/ItemsData/Enums/E_ItemSlot Enum" :default "NewEnumerator0"))
  (returns (ReturnValue :type "/Game/RPG_InventorySystem/Classes/Equippable/BP_BaseEquippable Object Reference"))
  (bind _returnvalue (select `/Game/RPG_InventorySystem/ItemsData/Enums/E_ItemSlot` Slot :`NewEnumerator7` (`self.Equipped Weapon Slot`) :`NewEnumerator12` (`self.Equipped Shield Slot`)))
  (`/Engine/EditorBlueprintResources/StandardMacros.IsValid` _returnvalue
    (:`Is Valid`
      (return _returnvalue))))

(fn `Get Item by Equipment Slot`
  (params (Slot :type "/Game/RPG_InventorySystem/ItemsData/Enums/E_ItemSlot Enum" :default "NewEnumerator0"))
  (returns (IsValid :type Boolean) (`Item Data` :type "/Game/RPG_InventorySystem/ItemsData/Structs/Item/S_ItemData Structure"))
  (bind (_value _returnvalue) (`BlueprintMapLibrary.Map_Find` (`self.Equipment Data`) Slot))
  (if _returnvalue
    (`/Game/RPG_InventorySystem/Blueprints/BML_Inventory.Is Item Class Valid?` _value
      (:`Valid`
        (return true _value))
      (:`Not Valid`
        (return false _value)))
    (else
      (return false))))

(fn `Get Item by ID`
  (params (`Item ID` :type String))
  (returns (Item :type "/Game/RPG_InventorySystem/ItemsData/Structs/Item/S_ItemData Structure") (Found :type Boolean))
  (bind _values (`BlueprintMapLibrary.Map_Values` (`self.Equipment Data`)))
  (bind _item (`/Game/RPG_InventorySystem/Blueprints/BML_Inventory.Find Item by ID` _values (`local.Item ID`))
    (:`Found`
      (return _item true))
    (:`Not Found`
      (return (struct) false))))

(fn `Remove Item from Equipment Array`
  (params (`Item Data` :type "/Game/RPG_InventorySystem/ItemsData/Structs/Item/S_ItemData Structure"))
  (locals (`L Empty Data` :type "/Game/RPG_InventorySystem/ItemsData/Structs/Item/S_ItemData Structure"))
  (bind ((`EquipmentSlot_82_D8E166834B91EEF8631726AE76BDFFE0` _equipmentslot)) (break `/Game/RPG_InventorySystem/ItemsData/Structs/Item/S_ItemData` `Item Data`))
  ;[1 0 0.06858 0.493] SERVER: Remove Item from Equipment Data
  (`/Game/RPG_InventorySystem/Blueprints/BML_Inventory.Switch Has Owner Authority`
    (:`Authority`
      (`BlueprintMapLibrary.Map_Remove` (`self.Equipment Data`) _equipmentslot)
      (bind _structout (setmembers `/Game/RPG_InventorySystem/ItemsData/Structs/Item/S_ItemData` :`StructRef` (`local.L Empty Data`) :`Equipment Slot` _equipmentslot))
      (`BlueprintMapLibrary.Map_Add` (`self.Equipment Data`) _equipmentslot _structout)
      ;[1 0.9656 0 0.493] IF STANDALONE: Call Event Dispatcher
      (if (`KismetSystemLibrary.IsStandalone`)
        (`self.On Removed from Equipment` (`local.Item Data`))
        (else
          ;[0.1707 1 0 0.493] CLIENT: Update Item
          (`self.Client Update Removed Item` (`local.Item Data`)))))))

(fn `Remove Item Quantity`
  (params (`Item Data` :type "/Game/RPG_InventorySystem/ItemsData/Structs/Item/S_ItemData Structure") (Quantity :type Integer))
  (locals (`L Item Data` :type "/Game/RPG_InventorySystem/ItemsData/Structs/Item/S_ItemData Structure"))
  (bind _output_get (set `local.L Item Data` `Item Data`))
  (`/Engine/EditorBlueprintResources/StandardMacros.CompareInt` (`.Quantity_76_AD4B883E4427C3E60B4B22B072F4E7C9` (break `/Game/RPG_InventorySystem/ItemsData/Structs/Item/S_ItemData` _output_get)) (`local.Quantity`)
    (:`>`
      (`self.Remove Item from Equipment Array` (`local.L Item Data`))
      (bind _structout (setmembers `/Game/RPG_InventorySystem/ItemsData/Structs/Item/S_ItemData` :`StructRef` (`local.L Item Data`) :`Quantity` (- (`.Quantity_76_AD4B883E4427C3E60B4B22B072F4E7C9` (break `/Game/RPG_InventorySystem/ItemsData/Structs/Item/S_ItemData` (`local.L Item Data`))) (`local.Quantity`))))
      (`self.Add Item to Equipment Array` _structout (`.EquipmentSlot_82_D8E166834B91EEF8631726AE76BDFFE0` (break `/Game/RPG_InventorySystem/ItemsData/Structs/Item/S_ItemData` _structout))))
    (:`==`
      (`self.Remove Item from Equipment Array` (`local.Item Data`) :!label _label)
      (`self.Detach Item from Equipment` (`local.Item Data`)))
    (:`<`
      (goto _label))))

(fn `Spawn and Attach Equippable Actor`
  (params (`Item Data` :type "/Game/RPG_InventorySystem/ItemsData/Structs/Item/S_ItemData Structure") (`Owning Character` :type "/Game/RPG_InventorySystem/Blueprints/Player/BP_RPGInventoryCharacter Object Reference"))
  (locals (`L Equippable` :type "/Game/RPG_InventorySystem/Classes/Equippable/BP_BaseEquippable Class Reference"))
  (bind _item_data (`local.Item Data`))
  (bind _equipped_weapon_slot (`self.Equipped Weapon Slot`))
  (bind _owning_character (`local.Owning Character`))
  (bind _owning_character_2 (`local.Owning Character`))
  (bind _equipped_shield_slot (`self.Equipped Shield Slot`))
  (`/Game/RPG_InventorySystem/Blueprints/BML_Inventory.Switch Has Owner Authority`
    (:`Authority`
      (`/Game/RPG_InventorySystem/Blueprints/BML_Inventory.Is Item Class Valid?` _item_data
        (:`Valid`
          (`/Engine/EditorBlueprintResources/StandardMacros.IsValid` (`local.Owning Character`)
            (:`Is Valid`
              (set `local.L Equippable` (defaults `Object` (`.Class_81_28B5086542C7943CC83294BF5B57815A` (break `/Game/RPG_InventorySystem/ItemsData/Structs/Item/S_ItemData` _item_data))))
              (switch `/Game/RPG_InventorySystem/ItemsData/Enums/E_ItemSlot` (`.EquipmentSlot_82_D8E166834B91EEF8631726AE76BDFFE0` (break `/Game/RPG_InventorySystem/ItemsData/Structs/Item/S_ItemData` (`local.Item Data`)))
                (:`NewEnumerator7`
                  ;[1 0.7202 0 0.52 24] Spawn & Attach Weapon [Main-Hand]
                  (`/Engine/EditorBlueprintResources/StandardMacros.IsValid` _equipped_weapon_slot
                    (:`Is Valid`
                      (`Actor.K2_DestroyActor` _equipped_weapon_slot))
                    (:`Is Not Valid`
                      _))
                  (bind _returnvalue (`|SpawnActorFromClass` (`local.L Equippable`) (`Actor.GetTransform` _owning_character_2) "Undefined" "OverrideRootScale" _owning_character_2 null))
                  (bind _output_get (set `self.Equipped Weapon Slot` _returnvalue))
                  (`Actor.K2_AttachToComponent` _output_get (`Character.Mesh` (`local.Owning Character`)) (select `/Game/RPG_InventorySystem/ItemsData/Enums/E_WeaponType` (defaults `Object` (`.Class_81_28B5086542C7943CC83294BF5B57815A` (break `/Game/RPG_InventorySystem/ItemsData/Structs/Item/S_ItemData` (`local.Item Data`)))) :`NewEnumerator3` "main_hand" :`NewEnumerator0` "main_hand" :`NewEnumerator1` "two_hand" :`NewEnumerator2` "main_hand" :!type "Name") "SnapToTarget" "SnapToTarget" "SnapToTarget" false))
                (:`NewEnumerator12`
                  ;[1 0.3392 0 0.52 24] Spawn & Attach Shield [Off-Hand]
                  (`/Engine/EditorBlueprintResources/StandardMacros.IsValid` _equipped_shield_slot
                    (:`Is Valid`
                      (`Actor.K2_DestroyActor` _equipped_shield_slot))
                    (:`Is Not Valid`
                      _))
                  (bind _returnvalue_2 (`|SpawnActorFromClass` (`local.L Equippable`) (`Actor.GetTransform` _owning_character) "Undefined" "OverrideRootScale" _owning_character null))
                  (bind _output_get_2 (set `self.Equipped Shield Slot` _returnvalue_2))
                  (`Actor.K2_AttachToComponent` _output_get_2 (`Character.Mesh` (`local.Owning Character`)) (select `/Game/RPG_InventorySystem/ItemsData/Enums/E_WeaponType` (defaults `Object` (`.Class_81_28B5086542C7943CC83294BF5B57815A` (break `/Game/RPG_InventorySystem/ItemsData/Structs/Item/S_ItemData` (`local.Item Data`)))) :`NewEnumerator3` "shield" :`NewEnumerator0` "off_hand" :`NewEnumerator1` "two_hand" :`NewEnumerator2` "shield" :!type "Name") "SnapToTarget" "SnapToTarget" "SnapToTarget" false))))))))))

(fn `Transfer Item from Equipment to Equipment`
  (params (`Dragged Data` :type "/Game/RPG_InventorySystem/ItemsData/Structs/Item/S_ItemData Structure") (`InSlot Data` :type "/Game/RPG_InventorySystem/ItemsData/Structs/Item/S_ItemData Structure"))
  (locals (`L Dragged Data` :type "/Game/RPG_InventorySystem/ItemsData/Structs/Item/S_ItemData Structure") (`L InSlot Data` :type "/Game/RPG_InventorySystem/ItemsData/Structs/Item/S_ItemData Structure"))
  (set `local.L Dragged Data` `Dragged Data`)
  (bind _output_get (set `local.L InSlot Data` `InSlot Data`))
  ;[1 0 0.01364 0.436] Is Slot not Empty?
  (`/Game/RPG_InventorySystem/Blueprints/BML_Inventory.Is Item Class Valid?` _output_get
    (:`Valid`
      (`self.Remove Item from Equipment Array` (`local.L InSlot Data`))
      (`self.Add Item to Equipment Array` (`local.Dragged Data`) (`.EquipmentSlot_82_D8E166834B91EEF8631726AE76BDFFE0` (break `/Game/RPG_InventorySystem/ItemsData/Structs/Item/S_ItemData` (`local.L InSlot Data`))))
      (`self.Remove Item from Equipment Array` (`local.L Dragged Data`))
      (`self.Add Item to Equipment Array` (`local.InSlot Data`) (`.EquipmentSlot_82_D8E166834B91EEF8631726AE76BDFFE0` (break `/Game/RPG_InventorySystem/ItemsData/Structs/Item/S_ItemData` (`local.L Dragged Data`))))
      (`self.Attach Item to Equipment` (`local.InSlot Data`))
      (`self.Attach Item to Equipment` (`local.Dragged Data`)))
    (:`Not Valid`
      (`self.Remove Item from Equipment Array` (`local.L Dragged Data`))
      (`self.Detach Item from Equipment` (`local.L Dragged Data`))
      (`self.Add Item to Equipment Array` (`local.L Dragged Data`) (`.EquipmentSlot_82_D8E166834B91EEF8631726AE76BDFFE0` (break `/Game/RPG_InventorySystem/ItemsData/Structs/Item/S_ItemData` (`local.L InSlot Data`))))
      (`self.Attach Item to Equipment` (`local.L Dragged Data`)))))

(fn `Transfer Item from Inventory to Equipment`
  (params (`Item Data` :type "/Game/RPG_InventorySystem/ItemsData/Structs/Item/S_ItemData Structure") (`InSlot Data` :type "/Game/RPG_InventorySystem/ItemsData/Structs/Item/S_ItemData Structure") (Inventory :type "/Game/RPG_InventorySystem/Blueprints/Components/AC_InventoryCore Object Reference") (Method :type "/Game/RPG_InventorySystem/ItemsData/Enums/E_InputMethod Enum" :default "NewEnumerator0"))
  (returns (Success :type Boolean) (`Failure Message` :type Text))
  (locals (`L InSlot Data` :type "/Game/RPG_InventorySystem/ItemsData/Structs/Item/S_ItemData Structure") (`L Item Data` :type "/Game/RPG_InventorySystem/ItemsData/Structs/Item/S_ItemData Structure"))
  (bind (_return_value _failure_message) (`self.Can Item be Equipped?` (`local.L Item Data`)))
  (set `local.L Item Data` `Item Data`)
  (set `local.L InSlot Data` `InSlot Data`)
  (if _return_value
    (switch `/Game/RPG_InventorySystem/ItemsData/Enums/E_InputMethod` (`local.Method`)
      (:`NewEnumerator0`
        ;[1 0 0.04044 0.384] Assign appropriate Item from Slot [Only if InSlot Data was not specified before - On Right Click]
        (bind _in_slot_data (`self.Assign Item from Equipment Slot` (`local.L Item Data`)))
        (set `local.L InSlot Data` _in_slot_data))
      (:`NewEnumerator1`
        _))
    (`/Game/RPG_InventorySystem/Blueprints/BML_Inventory.Is Item Class Valid?` (`local.L InSlot Data`) ; Not Valid = Empty
      (:`Valid`
        (`/Game/RPG_InventorySystem/Blueprints/BML_Inventory.Are Items the Same?` (`local.L Item Data`) (`local.L InSlot Data`)
          (:`True`
            (`/Game/RPG_InventorySystem/Blueprints/BML_Inventory.Are Items Stackable?` (`local.L Item Data`) (`local.L InSlot Data`)
              (:`True`
                ;[1 0.8785 0 0.488] Stack Items
                (`self.Add to Stack in Equipment` (`local.L Item Data`) (`.EquipmentSlot_82_D8E166834B91EEF8631726AE76BDFFE0` (break `/Game/RPG_InventorySystem/ItemsData/Structs/Item/S_ItemData` (`local.L InSlot Data`))))
                (`/Game/RPG_InventorySystem/Blueprints/Components/AC_InventoryCore.Remove Item from Inventory Array` (`local.Inventory`) (`local.L Item Data`))
                (return true ""))
              (:`False`
                _)))
          (:`False`
            _))
        ;[1 0 0 0.441] Swap Items
        (`self.Remove Item from Equipment Array` (`local.L InSlot Data`))
        (`/Game/RPG_InventorySystem/Blueprints/Components/AC_InventoryCore.Add Item to Inventory Array` (`local.Inventory`) (`local.L InSlot Data`) (`.Index_25_131A428548E5C72EF9A9C5B7F3185A4B` (break `/Game/RPG_InventorySystem/ItemsData/Structs/Item/S_ItemData` (`local.L Item Data`))))
        (`self.Add Item To Equipment Array` (`local.L Item Data`) (`.EquipmentSlot_82_D8E166834B91EEF8631726AE76BDFFE0` (break `/Game/RPG_InventorySystem/ItemsData/Structs/Item/S_ItemData` (`local.L InSlot Data`))))
        (`self.Detach Item from Equipment` (`local.L InSlot Data`))
        (`self.Attach Item to Equipment` (`local.L Item Data`))
        (`self.Try to Unequip associated Slot` (`local.L Item Data`) (`local.Inventory`))
        (return true ""))
      (:`Not Valid`
        ;[0.05725 1 0 0.399] Transfer Item to Empty Slot in Equipment
        (`/Game/RPG_InventorySystem/Blueprints/Components/AC_InventoryCore.Remove Item from Inventory Array` (`local.Inventory`) (`local.L Item Data`))
        (`self.Add Item To Equipment Array` (`local.L Item Data`) (`.EquipmentSlot_82_D8E166834B91EEF8631726AE76BDFFE0` (break `/Game/RPG_InventorySystem/ItemsData/Structs/Item/S_ItemData` (`local.L InSlot Data`))))
        (`self.Attach Item to Equipment` (`local.L Item Data`))
        (`self.Try to Unequip associated Slot` (`local.L Item Data`) (`local.Inventory`))
        (return true "")))
    (else
      (return false _failure_message))))

(fn `Try to Add to Partial Stack`
  (params (`Item Data` :type "/Game/RPG_InventorySystem/ItemsData/Structs/Item/S_ItemData Structure"))
  (returns (Success :type Boolean))
  (bind _values (`BlueprintMapLibrary.Map_Values` (`self.Equipment Data`)))
  (bind _slot_index (`/Game/RPG_InventorySystem/Blueprints/BML_Inventory.Has Partial Stack?` _values (`local.Item Data`))
    (:`True`
      (`self.Add to Stack in Equipment` (`local.Item Data`) (`.EquipmentSlot_82_D8E166834B91EEF8631726AE76BDFFE0` (break `/Game/RPG_InventorySystem/ItemsData/Structs/Item/S_ItemData` (`|GetArrayItem` _values _slot_index))))
      (return true))
    (:`False`
      (return false))))

(fn `Try to Unequip associated Slot`
  (params (`Item Data` :type "/Game/RPG_InventorySystem/ItemsData/Structs/Item/S_ItemData Structure") (Inventory :type "/Game/RPG_InventorySystem/Blueprints/Components/AC_InventoryCore Object Reference"))
  (locals (`L Associated Slot` :type "/Game/RPG_InventorySystem/ItemsData/Enums/E_ItemSlot Enum"))
  (bind (_isvalid _item_data) (`self.Get Item by Equipment Slot` (`local.L Associated Slot`)))
  (bind (_isvalid_2 _item_data_2) (`self.Get Item by Equipment Slot` (`local.L Associated Slot`)))
  (if (`self.Enable Off-Hand`)
    (set `local.L Associated Slot` (select `/Game/RPG_InventorySystem/ItemsData/Enums/E_ItemSlot` (`.EquipmentSlot_82_D8E166834B91EEF8631726AE76BDFFE0` (break `/Game/RPG_InventorySystem/ItemsData/Structs/Item/S_ItemData` `Item Data`)) :`NewEnumerator0` "NewEnumerator0" :`NewEnumerator1` "NewEnumerator0" :`NewEnumerator2` "NewEnumerator0" :`NewEnumerator3` "NewEnumerator0" :`NewEnumerator4` "NewEnumerator0" :`NewEnumerator5` "NewEnumerator0" :`NewEnumerator6` "NewEnumerator0" :`NewEnumerator7` "NewEnumerator12" :`NewEnumerator12` "NewEnumerator7" :`NewEnumerator8` "NewEnumerator0" :`NewEnumerator9` "NewEnumerator0" :`NewEnumerator10` "NewEnumerator0" :`NewEnumerator11` "NewEnumerator0" :`NewEnumerator13` "NewEnumerator0" :!type "/Game/RPG_InventorySystem/ItemsData/Enums/E_ItemSlot Enum"))
    (switch `/Game/RPG_InventorySystem/ItemsData/Enums/E_WeaponType` (defaults `Object` (`.Class_81_28B5086542C7943CC83294BF5B57815A` (break `/Game/RPG_InventorySystem/ItemsData/Structs/Item/S_ItemData` (`local.Item Data`))))
      (:`NewEnumerator0`
        ;[1 0.07874 0 0.478] Check if Two Hand is in the Associated Slot. If so - Remove it
        (if _isvalid :!label _label
          (if (`|EnumEquality` (defaults `Object` (`.Class_81_28B5086542C7943CC83294BF5B57815A` (break `/Game/RPG_InventorySystem/ItemsData/Structs/Item/S_ItemData` _item_data))) "NewEnumerator1")
            (bind (_success _failure_message) (`/Game/RPG_InventorySystem/Blueprints/Components/AC_InventoryCore.Transfer Item from Equipment` :`self` (`local.Inventory`) :`Item Data` _item_data :`Sender` self))
            (`/Game/RPG_InventorySystem/Blueprints/Components/AC_InventoryCore.Client Transfer Item Return Value` (`local.Inventory`) _success _failure_message))))
      (:`NewEnumerator1`
        ;[1 0.3781 0 0.598] Check if anything is in the Shield Slot. If so - Remove it
        (if _isvalid_2
          (bind (_success_2 _failure_message_2) (`/Game/RPG_InventorySystem/Blueprints/Components/AC_InventoryCore.Transfer Item from Equipment` :`self` (`local.Inventory`) :`Item Data` _item_data_2 :`Sender` self))
          (`/Game/RPG_InventorySystem/Blueprints/Components/AC_InventoryCore.Client Transfer Item Return Value` (`local.Inventory`) _success_2 _failure_message_2)))
      (:`NewEnumerator2`
        (goto _label)))))

(fn `Update Added Item`
  (params (`Item Data` :type "/Game/RPG_InventorySystem/ItemsData/Structs/Item/S_ItemData Structure"))
  (`BlueprintMapLibrary.Map_Add` (`self.Equipment Data`) (`.EquipmentSlot_82_D8E166834B91EEF8631726AE76BDFFE0` (break `/Game/RPG_InventorySystem/ItemsData/Structs/Item/S_ItemData` `Item Data`)) `Item Data`)
  (`self.On Added to Equipment` (`local.Item Data`))
  (`self.On Item Attach` (`local.Item Data`)))

(fn `Update Removed Item`
  (params (`Item Data` :type "/Game/RPG_InventorySystem/ItemsData/Structs/Item/S_ItemData Structure"))
  (locals (`L Empty Data` :type "/Game/RPG_InventorySystem/ItemsData/Structs/Item/S_ItemData Structure"))
  (bind ((`EquipmentSlot_82_D8E166834B91EEF8631726AE76BDFFE0` _equipmentslot)) (break `/Game/RPG_InventorySystem/ItemsData/Structs/Item/S_ItemData` `Item Data`))
  (`BlueprintMapLibrary.Map_Remove` (`self.Equipment Data`) _equipmentslot)
  (bind _structout (setmembers `/Game/RPG_InventorySystem/ItemsData/Structs/Item/S_ItemData` :`StructRef` (`local.L Empty Data`) :`Equipment Slot` _equipmentslot))
  (`BlueprintMapLibrary.Map_Add` (`self.Equipment Data`) _equipmentslot _structout)
  (`self.On Removed from Equipment` (`local.Item Data`))
  (`self.On Item Detach` (`local.Item Data`)))