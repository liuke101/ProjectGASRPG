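; Actor component for the RPG inventory system that handles quicksaving and the Load Game window.
; Quicksave requires Standalone mode and a free slot, then shows a save widget and saves through the GameInstance, with optional scene capture.
; The load window toggles input mode, cursor and move/look input, reporting widget state to the owner through messages.
; CanSave's "cannot save now" condition is a hardcoded true placeholder.
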(event `Quick Save Game`
  ;[1 0 0.01922 0.279] Save Data to Slot Type=Quicksave
  (bind (_return_value _failure_message) (`self.Can Save?`))
  (if _return_value
    (bind _asrpginventory_game_instance (cast `/Game/RPG_InventorySystem/Blueprints/SaveSystem/RPGInventory_GameInstance` (`GameplayStatics.GetGameInstance`)))
    (if (not (`/Game/RPG_InventorySystem/Blueprints/SaveSystem/RPGInventory_GameInstance.Does exceed Slot Limit?` _asrpginventory_game_instance (`self.Slots Limit`)))
      (bind _returnvalue (`|CreateWidget` "/Game/RPG_InventorySystem/UI/SaveSystem/WB_QuickSave.WB_QuickSave_C"))
      (`UserWidget.AddToViewport` _returnvalue 1)
      (`/Game/RPG_InventorySystem/Blueprints/SaveSystem/RPGInventory_GameInstance.Save Data to Slot` _asrpginventory_game_instance "NewEnumerator0" true "" (`self.Capture Scene on Quicksave`))
      (else
        (message `/Game/RPG_InventorySystem/Blueprints/BPI_WidgetManager.Display Message Notify` (`self.GetOwner`) "Slot limit exceeded.")))
    (else
      (message `/Game/RPG_InventorySystem/Blueprints/BPI_WidgetManager.Display Message Notify` (`self.GetOwner`) _failure_message))))

(event `Input Load Game`
  ;[1 0 0.01922 0.279] On Pressed Input 'LoadGame'
  (if (`self.Is LoadGameWindow Open?`)
    (`self.Close LoadGame Widget`)
    (else
      (message `/Game/RPG_InventorySystem/Blueprints/BPI_WidgetManager.Switch Widget to` (`self.GetOwner`) "NewEnumerator6"))))

(fn `Can Save?`
  (returns (`Return Value` :type Boolean) (`Failure Message` :type Text))
  (if (`KismetSystemLibrary.IsStandalone`)
    (if true
      (return true "")
      (else
        (return false "You cannot save now.")))
    (else
      (return false "Saving works only in Standalone mode."))))

(fn `Close LoadGame Widget`
  (bind _returnvalue (`self.GetOwner`))
  (bind _returnvalue_2 (`GameplayStatics.GetPlayerController` 0))
  (bind _loadgamewindow_ref (`self.LoadGameWindow Ref`))
  (set `self.Is LoadGameWindow Open?` false)
  (message `/Game/RPG_InventorySystem/Blueprints/BPI_WidgetManager.Set Active Widget` _returnvalue "NewEnumerator0")
  (message `/Game/RPG_InventorySystem/Blueprints/BPI_WidgetManager.Set Active Tab` _returnvalue "NewEnumerator0")
  (`/Engine/EditorBlueprintResources/StandardMacros.IsValid` _loadgamewindow_ref
    (:`Is Valid`
      (`Widget.RemoveFromParent` _loadgamewindow_ref))
    (:`Is Not Valid`
      _))
  (`WidgetBlueprintLibrary.SetInputMode_GameOnly` _returnvalue_2)
  (set `PlayerController.bShowMouseCursor` false _returnvalue_2)
  (`Controller.ResetIgnoreInputFlags` _returnvalue_2))

(fn `Open LoadGame Widget`
  (bind _returnvalue (`GameplayStatics.GetPlayerController` 0))
  (bind _returnvalue_2 (`self.GetOwner`))
  (`/Game/RPG_InventorySystem/Blueprints/BFL_Inventory.Play Sound On Opening Widget`)
  (set `self.Is LoadGameWindow Open?` true)
  (message `/Game/RPG_InventorySystem/Blueprints/BPI_WidgetManager.Set Active Widget` _returnvalue_2 "NewEnumerator6")
  (message `/Game/RPG_InventorySystem/Blueprints/BPI_WidgetManager.Set Active Tab` _returnvalue_2 "NewEnumerator6")
  (bind _returnvalue_3 (`|CreateWidget` "/Game/RPG_InventorySystem/UI/SaveSystem/WB_LoadGameWindow.WB_LoadGameWindow_C"))
  (bind _output_get (set `self.LoadGameWindow Ref` _returnvalue_3))
  (`UserWidget.AddToViewport` _output_get 1)
  (`WidgetBlueprintLibrary.SetInputMode_GameAndUIEx` _returnvalue (`self.LoadGameWindow Ref`))
  (set `PlayerController.bShowMouseCursor` true _returnvalue)
  ;[1 1 1] Ignore Move & Look Inputs
  (`Controller.SetIgnoreMoveInput` _returnvalue true)
  (`Controller.SetIgnoreLookInput` _returnvalue true))