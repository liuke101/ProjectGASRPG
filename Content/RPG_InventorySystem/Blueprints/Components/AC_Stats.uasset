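; Actor component that holds a character's stats, such as health, stamina, armor and damage, in a map for the RPG inventory system.
; Add, remove and set run on authority, clamp Health and Stamina to their max stats, and push results to the client, which broadcasts changes.
; Client initialization binds to the owner's equipment component; item stat helpers send class-default modifiers through server events.
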(event `Initialize Stats`
  ;[1 0 0.04033 0.587] Initialize Stats Component [Event called from Owner]
  (`self.Client Initialize Stats`))

(event `Client Initialize Stats`
  (bind _returnvalue (`Actor.GetComponentByClass` (`self.GetOwner`) "/Game/RPG_InventorySystem/Blueprints/Components/AC_PlayerEquipment.AC_PlayerEquipment_C"))
  ;[1 0.01447 0 0.561] CLIENT: Initialize Stats Component
  (`self.On Refresh Stats`)
  (`/Engine/EditorBlueprintResources/StandardMacros.IsValid` _returnvalue
    (:`Is Valid`
      (set `self.Owner Equipment` _returnvalue)
      (add `/Game/RPG_InventorySystem/Blueprints/Components/AC_PlayerEquipment.On Added to Equipment` (`self.Owner Equipment`) (`|CreateDelegate` :!event `Add Item Stats`))
      (add `/Game/RPG_InventorySystem/Blueprints/Components/AC_PlayerEquipment.On Removed from Equipment` (`self.Owner Equipment`) (`|CreateDelegate` :!event `Remove Item Stats`)))))

(event `Server Add Stat Value`
  (params (Stat :type "/Game/RPG_InventorySystem/ItemsData/Enums/E_StatCategory Enum" :default "NewEnumerator8") (Value :type "Float (double-precision)"))
  ;[0.1198 0.1198 0.1198 0.525] Server Events
  (`self.Add Stat Value` Stat Value))

(event `Client Stat Value Changed`
  (params (Stat :type "/Game/RPG_InventorySystem/ItemsData/Enums/E_StatCategory Enum" :default "NewEnumerator8") (`Stat Value` :type "Float (double-precision)"))
  ;[0.1198 0.1198 0.1198 0.525] Client Events
  (`BlueprintMapLibrary.Map_Add` (`self.Stats`) Stat `Stat Value`)
  (`self.On Changed Stat Value` Stat `Stat Value`))

(event `Server Remove Stat Value`
  (params (Stat :type "/Game/RPG_InventorySystem/ItemsData/Enums/E_StatCategory Enum" :default "NewEnumerator8") (Value :type "Float (double-precision)"))
  ;[0.1198 0.1198 0.1198 0.525] Server Events
  (`self.Remove Stat Value` Stat Value))

(event `Server Set Stat Value`
  (params (Stat :type "/Game/RPG_InventorySystem/ItemsData/Enums/E_StatCategory Enum" :default "NewEnumerator8") (Value :type "Float (double-precision)"))
  ;[0.1198 0.1198 0.1198 0.525] Server Events
  (`self.Set Stat Value` Stat Value))

(fn `Add Item Stats`
  (params (`Item Data` :type "/Game/RPG_InventorySystem/ItemsData/Structs/Item/S_ItemData Structure"))
  (for _array_element (defaults `Object` (`.Class_81_28B5086542C7943CC83294BF5B57815A` (break `/Game/RPG_InventorySystem/ItemsData/Structs/Item/S_ItemData` `Item Data`)))
    (`self.Server Add Stat Value` (break `/Game/RPG_InventorySystem/ItemsData/Structs/Item/S_ItemsStatRow` _array_element) (`.Value_5_4906130D4D518747DCD068861936DDBC` (break `/Game/RPG_InventorySystem/ItemsData/Structs/Item/S_ItemsStatRow` _array_element)))))

(fn `Add Stat Value`
  (params (Stat :type "/Game/RPG_InventorySystem/ItemsData/Enums/E_StatCategory Enum" :default "NewEnumerator8") (Value :type "Float (double-precision)"))
  (bind (_value _returnvalue) (`BlueprintMapLibrary.Map_Find` (`self.Stats`) (`local.Stat`)))
  (`/Game/RPG_InventorySystem/Blueprints/BML_Inventory.Switch Has Owner Authority`
    (:`Authority`
      (if _returnvalue
        (`BlueprintMapLibrary.Map_Add` (`self.Stats`) (`local.Stat`) (`self.Clamp Stat Value` (`local.Stat`) (+ _value (`local.Value`))))
        (`self.Client Stat Value Changed` (`local.Stat`) (`BlueprintMapLibrary.Map_Find` (`self.Stats`) (`local.Stat`)))))))

(fn `Clamp Stat Value`
  (params (Stat :type "/Game/RPG_InventorySystem/ItemsData/Enums/E_StatCategory Enum" :default "NewEnumerator8") (Value :type "Float (double-precision)"))
  (returns (`Clamped Value` :type "Float (double-precision)"))
  (bind _value (`local.Value`))
  (if (or (`|EnumEquality` Stat "NewEnumerator0") (`|EnumEquality` Stat "NewEnumerator1"))
    (return (`KismetMathLibrary.FClamp` (`local.Value`) 0.0 (select `/Game/RPG_InventorySystem/ItemsData/Enums/E_StatCategory` (`local.Stat`) :`NewEnumerator0` (`self.Get Stat Value` "NewEnumerator6") :`NewEnumerator1` (`self.Get Stat Value` "NewEnumerator7"))))
    (else
      (return (`KismetMathLibrary.FClamp` _value 0.0 _value)))))

(fn `Fix Any Miscalculations`
  (locals (`L Stat` :type "/Game/RPG_InventorySystem/ItemsData/Enums/E_StatCategory Enum"))
  (bind _l_stat (`local.L Stat`))
  (for _array_element (`|MakeArray` "NewEnumerator0" "NewEnumerator1" :!type "/Game/RPG_InventorySystem/ItemsData/Enums/E_StatCategory Enum")
    (set `local.L Stat` _array_element)
    (bind _value (`self.Get Stat Value` (select `/Game/RPG_InventorySystem/ItemsData/Enums/E_StatCategory` _array_element :`NewEnumerator8` "NewEnumerator8" :`NewEnumerator0` "NewEnumerator6" :`NewEnumerator6` "NewEnumerator8" :`NewEnumerator1` "NewEnumerator7" :`NewEnumerator7` "NewEnumerator8" :`NewEnumerator2` "NewEnumerator8" :`NewEnumerator3` "NewEnumerator8" :`NewEnumerator4` "NewEnumerator8" :!type "/Game/RPG_InventorySystem/ItemsData/Enums/E_StatCategory Enum")))
    (if (> (`self.Get Stat Value` _array_element) _value)
      (`BlueprintMapLibrary.Map_Add` (`self.Stats`) _l_stat (`self.Clamp Stat Value` _l_stat _value))
      (`self.Client Stat Value Changed` (`local.L Stat`) (`BlueprintMapLibrary.Map_Find` (`self.Stats`) (`local.L Stat`))))))

(fn `Get Max Stat Value`
  (params (Stat :type "/Game/RPG_InventorySystem/ItemsData/Enums/E_StatCategory Enum" :default "NewEnumerator8"))
  (returns (Value :type "Float (double-precision)"))
  (bind _value (`self.Get Stat Value` "NewEnumerator7"))
  (bind _value_2 (`self.Get Stat Value` "NewEnumerator6"))
  (if (`.ReturnValue` (`BlueprintMapLibrary.Map_Find` (`self.Stats`) Stat))
    (return (select `/Game/RPG_InventorySystem/ItemsData/Enums/E_StatCategory` Stat :`NewEnumerator0` _value_2 :`NewEnumerator6` _value_2 :`NewEnumerator1` _value :`NewEnumerator7` _value :`NewEnumerator2` 999.0 :`NewEnumerator3` 999.0 :`NewEnumerator4` 999.0))
    (else
      (return 0.0))))

(fn `Get Stat Value`
  (params (Stat :type "/Game/RPG_InventorySystem/ItemsData/Enums/E_StatCategory Enum" :default "NewEnumerator8"))
  (returns (Value :type "Float (double-precision)"))
  (bind (_value _returnvalue) (`BlueprintMapLibrary.Map_Find` (`self.Stats`) Stat))
  (if _returnvalue
    (return _value)
    (else
      (return 0.0))))

(fn `Remove Item Stats`
  (params (`Item Data` :type "/Game/RPG_InventorySystem/ItemsData/Structs/Item/S_ItemData Structure"))
  (for _array_element (defaults `Object` (`.Class_81_28B5086542C7943CC83294BF5B57815A` (break `/Game/RPG_InventorySystem/ItemsData/Structs/Item/S_ItemData` `Item Data`)))
    (`self.Server Remove Stat Value` (break `/Game/RPG_InventorySystem/ItemsData/Structs/Item/S_ItemsStatRow` _array_element) (`.Value_5_4906130D4D518747DCD068861936DDBC` (break `/Game/RPG_InventorySystem/ItemsData/Structs/Item/S_ItemsStatRow` _array_element)))))

(fn `Remove Stat Value`
  (params (Stat :type "/Game/RPG_InventorySystem/ItemsData/Enums/E_StatCategory Enum" :default "NewEnumerator8") (Value :type "Float (double-precision)"))
  (bind (_value _returnvalue) (`BlueprintMapLibrary.Map_Find` (`self.Stats`) (`local.Stat`)))
  (`/Game/RPG_InventorySystem/Blueprints/BML_Inventory.Switch Has Owner Authority`
    (:`Authority`
      (if _returnvalue
        (`BlueprintMapLibrary.Map_Add` (`self.Stats`) (`local.Stat`) (`self.Clamp Stat Value` (`local.Stat`) (- _value (`local.Value`))))
        (`self.Client Stat Value Changed` (`local.Stat`) (`BlueprintMapLibrary.Map_Find` (`self.Stats`) (`local.Stat`)))
        (`self.Fix Any Miscalculations`)))))

(fn `Set Stat Value`
  (params (Stat :type "/Game/RPG_InventorySystem/ItemsData/Enums/E_StatCategory Enum" :default "NewEnumerator8") (Value :type "Float (double-precision)"))
  (`/Game/RPG_InventorySystem/Blueprints/BML_Inventory.Switch Has Owner Authority`
    (:`Authority`
      (if (`.ReturnValue` (`BlueprintMapLibrary.Map_Find` (`self.Stats`) (`local.Stat`)))
        (`BlueprintMapLibrary.Map_Add` (`self.Stats`) (`local.Stat`) (`self.Clamp Stat Value` (`local.Stat`) (`local.Value`)))
        (`self.Client Stat Value Changed` (`local.Stat`) (`BlueprintMapLibrary.Map_Find` (`self.Stats`) (`local.Stat`)))
        (`self.Fix Any Miscalculations`)))))