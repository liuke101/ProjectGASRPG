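; Actor component from an RPG inventory system that tracks its owner's experience and level, with server-authoritative changes.
; On BeginPlay or Initialize it builds a level-to-required-experience map from a data table.
; Added experience triggers recursive level-ups that carry surplus over, clamping when no next level exists.
; Client events broadcast gains and level-ups, while RepNotify functions refresh the experience cap and broadcast level and experience changes.
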(event `self.ReceiveBeginPlay`
  (bind (_value _returnvalue) (`BlueprintMapLibrary.Map_Find` (`self.Leveling Data`) (`self.Current Level`)))
  ;[1 0.01447 0 0.561] Initialize: Setup Data and Max Experience
  (`self.Setup Leveling Data` :!label _label)
  (if _returnvalue
    (set `self.Level Max Experience` _value)
    (else
      (`KismetSystemLibrary.PrintString` "Current Level is not Valid!" true true (struct :`R` 1.0 :`B` 0.023868 :`A` 1.0) 5.0))))

(event `Event Initialize`
  ;[1 0.01447 0 0.561] Initialize: Setup Data and Max Experience
  (goto _label))

(event `Server Add Level Exp`
  (params (`Exp to Add` :type "Float (double-precision)"))
  ;[0.1198 0.1198 0.1198 0.525] Server Events
  (`self.Add Level Exp` `Exp to Add`))

(event `Client Gained Exp`
  (params (`Exp Gained` :type "Float (double-precision)"))
  ;[0.1198 0.1198 0.1198 0.525] Client Events
  (`self.On Gained Experience` `Exp Gained`))

(event `Server Increase Current Level`
  ;[0.1198 0.1198 0.1198 0.525] Server Events
  (`self.Increase Current Level`))

(event `Client Level Up`
  (params (`New Level` :type Integer))
  ;[0.1198 0.1198 0.1198 0.525] Client Events
  (`self.On Level Up` `New Level`))

(event `Server Set Current Level`
  (params (`New Level` :type Integer))
  ;[0.1198 0.1198 0.1198 0.525] Server Events
  (`self.Set Current Level` `New Level`))

(fn `Add Level Exp`
  (params (`Exp to Add` :type "Float (double-precision)"))
  (`/Game/RPG_InventorySystem/Blueprints/BML_Inventory.Switch Has Owner Authority`
    (:`Authority`
      (if (> `Exp to Add` 0.0)
        (set `self.Current Experience` (+ (`self.Current Experience`) `Exp to Add`))
        (`self.Client Gained Exp` `Exp to Add`)
        (if (`self.Exceed Level Max Exp?`)
          (`self.Increase Current Level`))))))

(fn `Exceed Level Max Exp?`
  (returns (`Return Value` :type Boolean))
  (return (>= (`self.Current Experience`) (`self.Level Max Experience`))))

(fn `Get Current Level`
  (returns (Level :type Integer))
  (return (`self.Current Level`)))

(fn `Increase Current Level`
  (`/Game/RPG_InventorySystem/Blueprints/BML_Inventory.Switch Has Owner Authority`
    (:`Authority`
      (if (`self.Exceed Level Max Exp?`)
        (if (`self.Is Next Level Valid?`)
          (set `self.Current Experience` (- (`self.Current Experience`) (`self.Level Max Experience`)))
          (bind _output_get (set `self.Current Level` (+ (`self.Current Level`) 1)))
          (`self.Client Level Up` _output_get)
          (if (`self.Exceed Level Max Exp?`)
            (`self.Increase Current Level`))
          (else
            (set `self.Current Experience` (`KismetMathLibrary.FClamp` (`self.Current Experience`) 0.0 (`self.Level Max Experience`)))))))))

(fn `Is Next Level Valid?`
  (returns (isValid :type Boolean))
  (return (`.ReturnValue` (`BlueprintMapLibrary.Map_Find` (`self.Leveling Data`) (+ (`self.Current Level`) 1)))))

(fn `OnRep_Current Experience`
  (`self.On Current Exp Changed`))

(fn `OnRep_Current Level`
  (set `self.Level Max Experience` (`BlueprintMapLibrary.Map_Find` (`self.Leveling Data`) (`self.Current Level`)))
  (`self.On Level Changed`))

(fn `Set Current Level`
  (params (`New Level` :type Integer))
  (`/Game/RPG_InventorySystem/Blueprints/BML_Inventory.Switch Has Owner Authority`
    (:`Authority`
      (if (`.ReturnValue` (`BlueprintMapLibrary.Map_Find` (`self.Leveling Data`) `New Level`))
        (set `self.Current Level` `New Level`)
        (set `self.Current Experience` 0.0)))))

(fn `Setup Leveling Data`
  (bind _leveling_datatable (`self.Leveling DataTable`))
  (bind _outrownames (`DataTableFunctionLibrary.GetDataTableRowNames` _leveling_datatable))
  (for _array_element _outrownames
    (bind _returnvalue (`|GetDataTableRow` _leveling_datatable _array_element)
      (:`then`
        (bind (_level _expneeded) (break `/Game/RPG_InventorySystem/ItemsData/Structs/S_LevelingSystem` _returnvalue))
        (`BlueprintMapLibrary.Map_Add` (`self.Leveling Data`) _level _expneeded)))))