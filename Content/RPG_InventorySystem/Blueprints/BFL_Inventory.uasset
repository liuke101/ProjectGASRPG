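; Blueprint function library of shared helpers for the RPG inventory system.
; Getters return the player character, camera and validity-checked inventory, equipment, crafting, interaction, leveling, stats, buff and saving components, plus an interactable owner's inventory.
; Item helpers filter arrays and sort them by type, rarity, value or weight, using class defaults to bucket or insertion-sort.
; Other helpers map gamepad icons and rarity colors, play UI sounds, add experience and toggle player capture.
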(fn `Add Level Exp to Player`
  (params (Target :type "Actor Object Reference") (`Exp to Add` :type "Float (double-precision)"))
  (bind _returnvalue (`Actor.GetComponentByClass` Target "/Game/RPG_InventorySystem/Blueprints/Components/AC_Leveling.AC_Leveling_C"))
  (`/Engine/EditorBlueprintResources/StandardMacros.IsValid` Target
    (:`Is Valid`
      (`/Engine/EditorBlueprintResources/StandardMacros.IsValid` _returnvalue
        (:`Is Valid`
          (`/Game/RPG_InventorySystem/Blueprints/Components/AC_Leveling.Server Add Level Exp` _returnvalue `Exp to Add`))))))

(fn `Get AC Consumable Buffs`
  (params (Target :type "Actor Object Reference"))
  (returns (ReturnValue :type "/Game/RPG_InventorySystem/Blueprints/Components/AC_ConsumableBuffs Object Reference"))
  (bind _returnvalue (`Actor.GetComponentByClass` Target "/Game/RPG_InventorySystem/Blueprints/Components/AC_ConsumableBuffs.AC_ConsumableBuffs_C"))
  (`/Engine/EditorBlueprintResources/StandardMacros.IsValid` _returnvalue
    (:`Is Valid`
      (return _returnvalue))
    (:`Is Not Valid`
      (return null))))

(fn `Get AC Crafting`
  (params (Target :type "Actor Object Reference"))
  (returns (AC_Crafting :type "/Game/RPG_InventorySystem/Blueprints/Components/AC_Crafting Object Reference"))
  (bind _returnvalue (`Actor.GetComponentByClass` Target "/Game/RPG_InventorySystem/Blueprints/Components/AC_Crafting.AC_Crafting_C"))
  (`/Engine/EditorBlueprintResources/StandardMacros.IsValid` _returnvalue
    (:`Is Valid`
      (return _returnvalue))
    (:`Is Not Valid`
      (return null))))

(fn `Get AC Interaction`
  (params (Target :type "Actor Object Reference"))
  (returns (`AC Interaction` :type "/Game/RPG_InventorySystem/Blueprints/Components/AC_Interaction Object Reference"))
  (bind _returnvalue (`Actor.GetComponentByClass` Target "/Game/RPG_InventorySystem/Blueprints/Components/AC_Interaction.AC_Interaction_C"))
  (`/Engine/EditorBlueprintResources/StandardMacros.IsValid` _returnvalue
    (:`Is Valid`
      (return _returnvalue))
    (:`Is Not Valid`
      (return null))))

(fn `Get AC Leveling`
  (params (Target :type "Actor Object Reference"))
  (returns (`Return Value` :type "/Game/RPG_InventorySystem/Blueprints/Components/AC_Leveling Object Reference"))
  (bind _returnvalue (`Actor.GetComponentByClass` Target "/Game/RPG_InventorySystem/Blueprints/Components/AC_Leveling.AC_Leveling_C"))
  (`/Engine/EditorBlueprintResources/StandardMacros.IsValid` _returnvalue
    (:`Is Valid`
      (return _returnvalue))
    (:`Is Not Valid`
      (return null))))

(fn `Get AC Saving`
  (params (Target :type "Actor Object Reference"))
  (returns (`Return Value` :type "/Game/RPG_InventorySystem/Blueprints/Components/AC_Saving Object Reference"))
  (bind _returnvalue (`Actor.GetComponentByClass` Target "/Game/RPG_InventorySystem/Blueprints/Components/AC_Saving.AC_Saving_C"))
  (`/Engine/EditorBlueprintResources/StandardMacros.IsValid` _returnvalue
    (:`Is Valid`
      (return _returnvalue))
    (:`Is Not Valid`
      (return null))))

(fn `Get AC Stats`
  (params (Target :type "Actor Object Reference"))
  (returns (ReturnValue :type "/Game/RPG_InventorySystem/Blueprints/Components/AC_Stats Object Reference"))
  (bind _returnvalue (`Actor.GetComponentByClass` Target "/Game/RPG_InventorySystem/Blueprints/Components/AC_Stats.AC_Stats_C"))
  (`/Engine/EditorBlueprintResources/StandardMacros.IsValid` _returnvalue
    (:`Is Valid`
      (return _returnvalue))
    (:`Is Not Valid`
      (return null))))

(fn `Get All Items of Type`
  (params (`Data Array` :type "Array of /Game/RPG_InventorySystem/ItemsData/Structs/Item/S_ItemData Structure") (`Item Type` :type "/Game/RPG_InventorySystem/ItemsData/Enums/E_ItemType Enum" :default "NewEnumerator0"))
  (returns (`Found Items` :type "Array of /Game/RPG_InventorySystem/ItemsData/Structs/Item/S_ItemData Structure"))
  (locals (Items :type "Array of /Game/RPG_InventorySystem/ItemsData/Structs/Item/S_ItemData Structure"))
  (for _array_element `Data Array`
    (`/Game/RPG_InventorySystem/Blueprints/BML_Inventory.Is Item Class Valid?` _array_element
      (:`Valid`
        (if (`|EnumEquality` (defaults `Object` (`.Class_81_28B5086542C7943CC83294BF5B57815A` (break `/Game/RPG_InventorySystem/ItemsData/Structs/Item/S_ItemData` _array_element))) (`local.Item Type`))
          (`KismetArrayLibrary.Array_Add` (`local.Items`) _array_element)))))
  (return (`local.Items`)))

(fn `Get Current Interactable Object`
  (params (Target :type "Actor Object Reference"))
  (returns (`Current Interactable` :type "/Game/RPG_InventorySystem/Blueprints/Components/AC_Interactable Object Reference"))
  (bind _returnvalue (`Actor.GetComponentByClass` Target "/Game/RPG_InventorySystem/Blueprints/Components/AC_Interaction.AC_Interaction_C"))
  (bind _current_interactable (`/Game/RPG_InventorySystem/Blueprints/Components/AC_Interaction.Current Interactable` _returnvalue))
  (`/Engine/EditorBlueprintResources/StandardMacros.IsValid` _returnvalue
    (:`Is Valid`
      (`/Engine/EditorBlueprintResources/StandardMacros.IsValid` _current_interactable
        (:`Is Valid`
          (return _current_interactable))
        (:`Is Not Valid`
          (return null))))
    (:`Is Not Valid`
      (return null))))

(fn `Get Gamepad Icon`
  (params (Input :type "/Game/RPG_InventorySystem/ItemsData/Enums/E_GamepadInputs Enum" :default "NewEnumerator0"))
  (returns (Icon :type "Texture2D Object Reference"))
  (return (select `/Game/RPG_InventorySystem/ItemsData/Enums/E_GamepadInputs` Input :`NewEnumerator0` "/Game/RPG_InventorySystem/Textures/Images/UILayout/GamepadIcons/T_Gamepad_A.T_Gamepad_A" :`NewEnumerator1` "/Game/RPG_InventorySystem/Textures/Images/UILayout/GamepadIcons/T_Gamepad_B.T_Gamepad_B" :`NewEnumerator2` "/Game/RPG_InventorySystem/Textures/Images/UILayout/GamepadIcons/T_Gamepad_X.T_Gamepad_X" :`NewEnumerator3` "/Game/RPG_InventorySystem/Textures/Images/UILayout/GamepadIcons/T_Gamepad_Y.T_Gamepad_Y" :`NewEnumerator4` "/Game/RPG_InventorySystem/Textures/Images/UILayout/GamepadIcons/T_Gamepad_LStick.T_Gamepad_LStick" :`NewEnumerator5` "/Game/RPG_InventorySystem/Textures/Images/UILayout/GamepadIcons/T_Gamepad_LStickDown.T_Gamepad_LStickDown" :`NewEnumerator6` "/Game/RPG_InventorySystem/Textures/Images/UILayout/GamepadIcons/T_Gamepad_RStick.T_Gamepad_RStick" :`NewEnumerator7` "/Game/RPG_InventorySystem/Textures/Images/UILayout/GamepadIcons/T_Gamepad_RStickDown.T_Gamepad_RStickDown" :`NewEnumerator8` "/Game/RPG_InventorySystem/Textures/Images/UILayout/GamepadIcons/T_Gamepad_LB.T_Gamepad_LB" :`NewEnumerator9` "/Game/RPG_InventorySystem/Textures/Images/UILayout/GamepadIcons/T_Gamepad_RB.T_Gamepad_RB" :`NewEnumerator10` "/Game/RPG_InventorySystem/Textures/Images/UILayout/GamepadIcons/T_Gamepad_LT.T_Gamepad_LT" :`NewEnumerator11` "/Game/RPG_InventorySystem/Textures/Images/UILayout/GamepadIcons/T_Gamepad_RT.T_Gamepad_RT" :`NewEnumerator12` "/Game/RPG_InventorySystem/Textures/Images/UILayout/GamepadIcons/T_Gamepad_DpadUp.T_Gamepad_DpadUp" :`NewEnumerator13` "/Game/RPG_InventorySystem/Textures/Images/UILayout/GamepadIcons/T_Gamepad_DpadDown.T_Gamepad_DpadDown" :`NewEnumerator14` "/Game/RPG_InventorySystem/Textures/Images/UILayout/GamepadIcons/T_Gamepad_DpadRight.T_Gamepad_DpadRight" :`NewEnumerator15` "/Game/RPG_InventorySystem/Textures/Images/UILayout/GamepadIcons/T_Gamepad_DpadLeft.T_Gamepad_DpadLeft" :`NewEnumerator16` "/Game/RPG_InventorySystem/Textures/Images/UILayout/GamepadIcons/T_Gamepad_ViewButton.T_Gamepad_ViewButton" :`NewEnumerator17` "/Game/RPG_InventorySystem/Textures/Images/UILayout/GamepadIcons/T_Gamepad_MenuButton.T_Gamepad_MenuButton" :!type "Texture2D Object Reference")))

(fn `Get Inventory from Interactable`
  (params (Interactable :type "/Game/RPG_InventorySystem/Blueprints/Components/AC_Interactable Object Reference"))
  (returns (IsValid :type Boolean) (Inventory :type "/Game/RPG_InventorySystem/Blueprints/Components/AC_InventoryCore Object Reference"))
  (bind _returnvalue (`Actor.GetComponentByClass` (`ActorComponent.GetOwner` Interactable) "/Game/RPG_InventorySystem/Blueprints/Components/AC_InventoryCore.AC_InventoryCore_C"))
  (`/Engine/EditorBlueprintResources/StandardMacros.IsValid` Interactable
    (:`Is Valid`
      (`/Engine/EditorBlueprintResources/StandardMacros.IsValid` _returnvalue
        (:`Is Valid`
          (return true _returnvalue))
        (:`Is Not Valid`
          _)))
    (:`Is Not Valid`
      _))
  (return false null))

(fn `Get Player Camera`
  (params (Target :type "Actor Object Reference"))
  (returns (Camera :type "CameraComponent Object Reference"))
  (bind _returnvalue (`Actor.GetComponentByClass` Target "/Script/Engine.CameraComponent"))
  (`/Engine/EditorBlueprintResources/StandardMacros.IsValid` _returnvalue
    (:`Is Valid`
      (return _returnvalue))
    (:`Is Not Valid`
      (return null))))

(fn `Get Player Equipment`
  (params (Target :type "Actor Object Reference"))
  (returns (ReturnValue :type "/Game/RPG_InventorySystem/Blueprints/Components/AC_PlayerEquipment Object Reference"))
  (bind _returnvalue (`Actor.GetComponentByClass` Target "/Game/RPG_InventorySystem/Blueprints/Components/AC_PlayerEquipment.AC_PlayerEquipment_C"))
  (`/Engine/EditorBlueprintResources/StandardMacros.IsValid` _returnvalue
    (:`Is Valid`
      (return _returnvalue))
    (:`Is Not Valid`
      (return null))))

(fn `Get Player Inventory`
  (params (Target :type "Actor Object Reference"))
  (returns (ReturnValue :type "/Game/RPG_InventorySystem/Blueprints/Components/AC_PlayerInventory Object Reference"))
  (bind _returnvalue (`Actor.GetComponentByClass` Target "/Game/RPG_InventorySystem/Blueprints/Components/AC_PlayerInventory.AC_PlayerInventory_C"))
  (`/Engine/EditorBlueprintResources/StandardMacros.IsValid` _returnvalue
    (:`Is Valid`
      (return _returnvalue))
    (:`Is Not Valid`
      (return null))))

(fn `Get Rarity Color`
  (params (Rarity :type "/Game/RPG_InventorySystem/ItemsData/Enums/E_ItemRarity Enum" :default "NewEnumerator7"))
  (returns (Color :type "SlateColor Structure"))
  (return (make `SlateColor` (select `/Game/RPG_InventorySystem/ItemsData/Enums/E_ItemRarity` Rarity :`NewEnumerator0` (struct :`R` 0.775822 :`G` 0.775822 :`B` 0.775822 :`A` 1.0) :`NewEnumerator2` (struct :`R` 0.046665 :`G` 0.291771 :`B` 0.14996 :`A` 1.0) :`NewEnumerator3` (struct :`R` 0.361307 :`B` 0.672443 :`A` 1.0) :`NewEnumerator4` (struct :`R` 0.564712 :`G` 0.417885 :`B` 0.039546 :`A` 1.0) :`NewEnumerator1` (struct :`R` 0.05448 :`G` 0.291771 :`B` 0.53948 :`A` 1.0) :`NewEnumerator5` (struct :`R` 0.665387 :`G` 0.274677 :`B` 0.082283 :`A` 1.0) :!type "LinearColor Structure"))))

(fn `Get RPGInventory Player Ref`
  (returns (Player :type "/Game/RPG_InventorySystem/Blueprints/Player/BP_RPGInventoryCharacter Object Reference"))
  (bind _asbp_rpginventory_character (cast `/Game/RPG_InventorySystem/Blueprints/Player/BP_RPGInventoryCharacter` (`GameplayStatics.GetPlayerCharacter` null))
    (:`then`
      (return _asbp_rpginventory_character))
    (:`CastFailed`
      (return null))))

(fn `Play Sound On Button Switched`
  (`GameplayStatics.PlaySound2D` null "/Game/RPG_InventorySystem/Sounds/S_Click.S_Click" 1.0 1.0 0.0 null null))

(fn `Play Sound On Consumable Used`
  (`GameplayStatics.PlaySound2D` null "/Game/RPG_InventorySystem/Sounds/S_Click.S_Click" 1.0 1.0 0.0 null null))

(fn `Play Sound On Item Crafted`
  (`GameplayStatics.PlaySound2D` null "/Game/RPG_InventorySystem/Sounds/S_Craft.S_Craft" 1.0 1.0 0.0 null null))

(fn `Play Sound On Item Dropped`
  (`GameplayStatics.PlaySound2D` null "/Game/RPG_InventorySystem/Sounds/S_Click.S_Click" 1.0 1.0 0.0 null null))

(fn `Play Sound On Item Picked Up`
  (`GameplayStatics.PlaySound2D` null "/Game/RPG_InventorySystem/Sounds/S_Pickup.S_Pickup" 1.0 1.0 0.0 null null))

(fn `Play Sound On Opening Widget`
  (`GameplayStatics.PlaySound2D` null "/Game/RPG_InventorySystem/Sounds/S_OpenWidget.S_OpenWidget" 1.0 1.0 0.0 null null))

(fn `Play Sound On Tab Switched`
  (`GameplayStatics.PlaySound2D` null "/Game/RPG_InventorySystem/Sounds/S_Switch.S_Switch" 0.6 1.0 0.0 null null))

(fn `Quick Sort Items`
  (params (`Data Array` :type "Array of /Game/RPG_InventorySystem/ItemsData/Structs/Item/S_ItemData Structure"))
  (returns (`Sorted Items` :type "Array of /Game/RPG_InventorySystem/ItemsData/Structs/Item/S_ItemData Structure"))
  (locals (Sorted :type "Array of /Game/RPG_InventorySystem/ItemsData/Structs/Item/S_ItemData Structure"))
  (for _array_element `Data Array`
    (`/Game/RPG_InventorySystem/Blueprints/BML_Inventory.Is Item Class Valid?` _array_element
      (:`Valid`
        (`KismetArrayLibrary.Array_Add` (`local.Sorted`) _array_element))))
  (return (`local.Sorted`)))

(fn `Sort Items by Rarity`
  (params (`Data Array` :type "Array of /Game/RPG_InventorySystem/ItemsData/Structs/Item/S_ItemData Structure"))
  (returns (`Sorted Items` :type "Array of /Game/RPG_InventorySystem/ItemsData/Structs/Item/S_ItemData Structure"))
  (locals (Common :type "Array of /Game/RPG_InventorySystem/ItemsData/Structs/Item/S_ItemData Structure") (Consumable :type "Array of /Game/RPG_InventorySystem/ItemsData/Structs/Item/S_ItemData Structure") (Superior :type "Array of /Game/RPG_InventorySystem/ItemsData/Structs/Item/S_ItemData Structure") (Epic :type "Array of /Game/RPG_InventorySystem/ItemsData/Structs/Item/S_ItemData Structure") (Legendary :type "Array of /Game/RPG_InventorySystem/ItemsData/Structs/Item/S_ItemData Structure") (Usable :type "Array of /Game/RPG_InventorySystem/ItemsData/Structs/Item/S_ItemData Structure") (Sorted :type "Array of /Game/RPG_InventorySystem/ItemsData/Structs/Item/S_ItemData Structure"))
  (for _array_element `Data Array`
    (`/Game/RPG_InventorySystem/Blueprints/BML_Inventory.Is Item Class Valid?` _array_element
      (:`Valid`
        (`KismetArrayLibrary.Array_Add` (select `/Game/RPG_InventorySystem/ItemsData/Enums/E_ItemRarity` (defaults `Object` (`.Class_81_28B5086542C7943CC83294BF5B57815A` (break `/Game/RPG_InventorySystem/ItemsData/Structs/Item/S_ItemData` _array_element))) :`NewEnumerator0` (`local.Common`) :`NewEnumerator2` (`local.Superior`) :`NewEnumerator3` (`local.Epic`) :`NewEnumerator4` (`local.Legendary`) :`NewEnumerator1` (`local.Consumable`) :`NewEnumerator5` (`local.Usable`)) _array_element))))
  (`KismetArrayLibrary.Array_Append` (`local.Sorted`) (`local.Legendary`))
  (`KismetArrayLibrary.Array_Append` (`local.Sorted`) (`local.Epic`))
  (`KismetArrayLibrary.Array_Append` (`local.Sorted`) (`local.Superior`))
  (`KismetArrayLibrary.Array_Append` (`local.Sorted`) (`local.Common`))
  (`KismetArrayLibrary.Array_Append` (`local.Sorted`) (`local.Consumable`))
  (`KismetArrayLibrary.Array_Append` (`local.Sorted`) (`local.Usable`))
  (return (`local.Sorted`)))

(fn `Sort Items by Type`
  (params (`Data Array` :type "Array of /Game/RPG_InventorySystem/ItemsData/Structs/Item/S_ItemData Structure"))
  (returns (`Sorted Items` :type "Array of /Game/RPG_InventorySystem/ItemsData/Structs/Item/S_ItemData Structure"))
  (locals (Other :type "Array of /Game/RPG_InventorySystem/ItemsData/Structs/Item/S_ItemData Structure") (QItems :type "Array of /Game/RPG_InventorySystem/ItemsData/Structs/Item/S_ItemData Structure") (CrIngredients :type "Array of /Game/RPG_InventorySystem/ItemsData/Structs/Item/S_ItemData Structure") (Potions :type "Array of /Game/RPG_InventorySystem/ItemsData/Structs/Item/S_ItemData Structure") (Food :type "Array of /Game/RPG_InventorySystem/ItemsData/Structs/Item/S_ItemData Structure") (Shields :type "Array of /Game/RPG_InventorySystem/ItemsData/Structs/Item/S_ItemData Structure") (Weapons :type "Array of /Game/RPG_InventorySystem/ItemsData/Structs/Item/S_ItemData Structure") (Armor :type "Array of /Game/RPG_InventorySystem/ItemsData/Structs/Item/S_ItemData Structure") (Sorted :type "Array of /Game/RPG_InventorySystem/ItemsData/Structs/Item/S_ItemData Structure") (Currency :type "Array of /Game/RPG_InventorySystem/ItemsData/Structs/Item/S_ItemData Structure"))
  (for _array_element `Data Array`
    (`/Game/RPG_InventorySystem/Blueprints/BML_Inventory.Is Item Class Valid?` _array_element
      (:`Valid`
        (`KismetArrayLibrary.Array_Add` (select `/Game/RPG_InventorySystem/ItemsData/Enums/E_ItemType` (defaults `Object` (`.Class_81_28B5086542C7943CC83294BF5B57815A` (break `/Game/RPG_InventorySystem/ItemsData/Structs/Item/S_ItemData` _array_element))) :`NewEnumerator1` (`local.Armor`) :`NewEnumerator2` (`local.Weapons`) :`NewEnumerator6` (`local.Shields`) :`NewEnumerator3` (`local.Food`) :`NewEnumerator4` (`local.Potions`) :`NewEnumerator7` (`local.CrIngredients`) :`NewEnumerator8` (`local.QItems`) :`NewEnumerator5` (`local.Other`) :`NewEnumerator9` (`local.Currency`)) _array_element))))
  ;[0.02042 0 1 0.133] Inventory P1
  (`KismetArrayLibrary.Array_Append` (`local.Sorted`) (`local.Armor`))
  (`KismetArrayLibrary.Array_Append` (`local.Sorted`) (`local.Weapons`))
  (`KismetArrayLibrary.Array_Append` (`local.Sorted`) (`local.Shields`))
  ;[0 1 0.8949 0.238] Inventory P2
  (`KismetArrayLibrary.Array_Append` (`local.Sorted`) (`local.Potions`))
  (`KismetArrayLibrary.Array_Append` (`local.Sorted`) (`local.Food`))
  ;[1 0.7568 0 0.17] Inventory P3
  (`KismetArrayLibrary.Array_Append` (`local.Sorted`) (`local.CrIngredients`))
  ;[1 0.3792 0 0.17] Inventory P4
  (`KismetArrayLibrary.Array_Append` (`local.Sorted`) (`local.QItems`))
  (`KismetArrayLibrary.Array_Append` (`local.Sorted`) (`local.Other`))
  ;[0 0 0 0.488] Non-Panel
  (`KismetArrayLibrary.Array_Append` (`local.Sorted`) (`local.Currency`))
  (return (`local.Sorted`)))

(fn `Sort Items by Value`
  (params (`Data Array` :type "Array of /Game/RPG_InventorySystem/ItemsData/Structs/Item/S_ItemData Structure"))
  (returns (`Sorted Items` :type "Array of /Game/RPG_InventorySystem/ItemsData/Structs/Item/S_ItemData Structure"))
  (locals (Sorted :type "Array of /Game/RPG_InventorySystem/ItemsData/Structs/Item/S_ItemData Structure") (Found :type Boolean))
  (for _array_element `Data Array`
    (`/Game/RPG_InventorySystem/Blueprints/BML_Inventory.Is Item Class Valid?` _array_element
      (:`Valid`
        (for (_array_element_2 _array_index) (`local.Sorted`)
          (if (> (defaults `Object` (`.Class_81_28B5086542C7943CC83294BF5B57815A` (break `/Game/RPG_InventorySystem/ItemsData/Structs/Item/S_ItemData` _array_element))) (defaults `Object` (`.Class_81_28B5086542C7943CC83294BF5B57815A` (break `/Game/RPG_InventorySystem/ItemsData/Structs/Item/S_ItemData` _array_element_2))))
            (`|ExecutionSequence`
              (:`then_0`
                (set `local.Found` true)
                (`KismetArrayLibrary.Array_Insert` (`local.Sorted`) _array_element _array_index))
              (:`then_1`
                (break)))))
        (if (`local.Found`)
          (set `local.Found` false)
          (else
            (`KismetArrayLibrary.Array_Add` (`local.Sorted`) _array_element))))))
  (return (`local.Sorted`)))

(fn `Sort Items by Weight`
  (params (`Data Array` :type "Array of /Game/RPG_InventorySystem/ItemsData/Structs/Item/S_ItemData Structure"))
  (returns (`Sorted Items` :type "Array of /Game/RPG_InventorySystem/ItemsData/Structs/Item/S_ItemData Structure"))
  (locals (Sorted :type "Array of /Game/RPG_InventorySystem/ItemsData/Structs/Item/S_ItemData Structure") (Found :type Boolean))
  (for _array_element `Data Array`
    (`/Game/RPG_InventorySystem/Blueprints/BML_Inventory.Is Item Class Valid?` _array_element
      (:`Valid`
        (for (_array_element_2 _array_index) (`local.Sorted`)
          (if (> (defaults `Object` (`.Class_81_28B5086542C7943CC83294BF5B57815A` (break `/Game/RPG_InventorySystem/ItemsData/Structs/Item/S_ItemData` _array_element))) (defaults `Object` (`.Class_81_28B5086542C7943CC83294BF5B57815A` (break `/Game/RPG_InventorySystem/ItemsData/Structs/Item/S_ItemData` _array_element_2))))
            (`|ExecutionSequence`
              (:`then_0`
                (set `local.Found` true)
                (`KismetArrayLibrary.Array_Insert` (`local.Sorted`) _array_element _array_index))
              (:`then_1`
                (break)))))
        (if (`local.Found`)
          (set `local.Found` false)
          (else
            (`KismetArrayLibrary.Array_Add` (`local.Sorted`) _array_element))))))
  (return (`local.Sorted`)))

(fn `Start Player Capture 2D`
  (params (Controller :type "Actor Object Reference"))
  (bind _asbp_rpginventory_player_controller (cast `/Game/RPG_InventorySystem/Blueprints/Player/BP_RPGInventoryPlayerController` Controller))
  (`/Game/RPG_InventorySystem/Blueprints/Player/BP_RPGInventoryPlayerController.Start Player Capture` _asbp_rpginventory_player_controller))

(fn `Stop Player Capture 2D`
  (params (Controller :type "Actor Object Reference"))
  (bind _asbp_rpginventory_player_controller (cast `/Game/RPG_InventorySystem/Blueprints/Player/BP_RPGInventoryPlayerController` Controller))
  (`/Game/RPG_InventorySystem/Blueprints/Player/BP_RPGInventoryPlayerController.Stop Player Capture` _asbp_rpginventory_player_controller))