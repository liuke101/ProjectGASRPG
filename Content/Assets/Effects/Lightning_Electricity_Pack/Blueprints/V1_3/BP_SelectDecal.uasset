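; Selection decal actor from a lightning effects pack that projects a tinted marker using M_SelectionDecal.
; Construction script scales the decal by Size and creates a dynamic material instance with color, boost and density.
; BeginPlay rebuilds that instance after a zero-second delay but does not reapply Density.
; An Animation timeline would drive the material's scale and radius parameters, but nothing starts it.
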(event `self.ReceiveBeginPlay`
  (bind _size (`self.Size`))
  (bind _decal (`self.Decal`))
  (bind _returnvalue (* 0.2 _size))
  (`KismetSystemLibrary.Delay` 0.0)
  ;[1 1 1] Decal Initialization
  (`DecalComponent.SetDecalMaterial` _decal "/Game/Assets/Effects/Lightning_Electricity_Pack/Materials/M_SelectionDecal.M_SelectionDecal")
  (`SceneComponent.SetWorldScale3D` _decal (`KismetMathLibrary.MakeVector` (* 0.12 _size) _returnvalue _returnvalue))
  (bind _returnvalue_2 (`KismetMaterialLibrary.CreateDynamicMaterialInstance` (`DecalComponent.DecalMaterial` _decal)))
  (bind _output_get (set `self.Material` _returnvalue_2))
  (`MaterialInstanceDynamic.SetVectorParameterValue` _output_get "Color" (`self.Color`))
  (`DecalComponent.SetDecalMaterial` (`self.Decal`) _returnvalue_2)
  (`MaterialInstanceDynamic.SetScalarParameterValue` _returnvalue_2 "Boost" (`self.ColorBoost`)))

(fn `UserConstructionScript`
  (bind _size (`self.Size`))
  (bind _decal (`self.Decal`))
  (bind _returnvalue (* 0.2 _size))
  ;[1 1 1] Decal Initialization
  (`DecalComponent.SetDecalMaterial` _decal "/Game/Assets/Effects/Lightning_Electricity_Pack/Materials/M_SelectionDecal.M_SelectionDecal")
  (`SceneComponent.SetWorldScale3D` _decal (`KismetMathLibrary.MakeVector` (* 0.12 _size) _returnvalue _returnvalue))
  (bind _returnvalue_2 (`KismetMaterialLibrary.CreateDynamicMaterialInstance` (`DecalComponent.DecalMaterial` _decal)))
  (bind _output_get (set `self.Material` _returnvalue_2))
  (`MaterialInstanceDynamic.SetVectorParameterValue` _output_get "Color" (`self.Color`))
  (`DecalComponent.SetDecalMaterial` (`self.Decal`) _returnvalue_2)
  (`MaterialInstanceDynamic.SetScalarParameterValue` _returnvalue_2 "Boost" (`self.ColorBoost`))
  (`MaterialInstanceDynamic.SetScalarParameterValue` _returnvalue_2 "Density" (`self.Density`)))