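; BP_EnemyBase is an enemy character base Blueprint that handles shared visual setup and combat hooks.
; Construction snaps the weapon to a mesh socket, enables custom depth stencil on both, and places the health bar above the capsule using its half-height.
; A timeline drives the DissolveValue material parameter for the death dissolve.
; The combat interface's UpdateFacingTarget event feeds a Motion Warping target so skill montages face their target.
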(event `self.ReceiveBeginPlay`
  (`parent.ReceiveBeginPlay`))

(event `self.ReceiveTick`
  (params (DeltaSeconds :type "Float (single-precision)"))
  (`parent.ReceiveTick` DeltaSeconds))

(event `self.StartMeshDissolveTimeline`
  (params (DynamicMaterialInstance :type "MaterialInstanceDynamic Object Reference"))
  ;[1 1 1] 死亡溶解
  (bind (_direction _dissolvetrack) (`Timeline|时间轴`)
    (:`Update`
      (`MaterialInstanceDynamic.SetScalarParameterValue` DynamicMaterialInstance "DissolveValue" _dissolvetrack))))

(event `CombatInterface.UpdateFacingTarget`
  (params (TargetLocation :type "Vector Structure (by ref)"))
  ;[0.5569 0.9661 1] CombatInterface
  ;;[1 0.6164 0.2701] MotionWarping:释放技能时，使Montage面向敌人
  (`MotionWarpingComponent.AddOrUpdateWarpTargetFromLocation` (`self.MotionWarping`) "FacingTarget" TargetLocation))

(fn `UserConstructionScript`
  (bind _mesh (`self.Mesh`))
  (`SceneComponent.K2_AttachToComponent` (`self.Weapon`) (`self.Mesh`) (`self.WeaponAttachSocket`) "SnapToTarget" "SnapToTarget" "SnapToTarget" true)
  (`PrimitiveComponent.SetRenderCustomDepth` _mesh true)
  (`PrimitiveComponent.SetRenderCustomDepth` (`self.Weapon`) true)
  (`PrimitiveComponent.SetCustomDepthStencilValue` _mesh 255)
  (`PrimitiveComponent.SetCustomDepthStencilValue` (`self.Weapon`) 255)
  ;[1 1 1] 设置HelathBar初始位置，根据胶囊体高度
  (`SceneComponent.K2_SetRelativeLocation` (`self.HealthBar`) (`KismetMathLibrary.MakeVector` 0.0 0.0 (+ (`CapsuleComponent.GetScaledCapsuleHalfHeight` (`self.CapsuleComponent`)) 100.0)) false false))