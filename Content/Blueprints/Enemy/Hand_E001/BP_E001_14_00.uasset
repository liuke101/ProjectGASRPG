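; BP_E001_14_00 is an enemy Blueprint in the Hand_E001 set that adds a debug visualization of its hand sockets.
; Every Tick it draws yellow debug spheres at the LeftHandSocket and RightHandSocket locations on its Mesh.
; BeginPlay and the construction script only call the parent, and the overlap event is disabled, so any other behavior comes from the parent class.
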(event `self.ReceiveBeginPlay`
  (`parent.ReceiveBeginPlay`))

(event `self.ReceiveTick`
  (params (DeltaSeconds :type "Float (single-precision)"))
  (`KismetSystemLibrary.DrawDebugSphere` (`SceneComponent.GetSocketLocation` (`self.Mesh`) "LeftHandSocket") 100.0 12 (struct :`R` 1.0 :`G` 0.99351 :`A` 1.0) 0.0 1.0)
  (`KismetSystemLibrary.DrawDebugSphere` (`SceneComponent.GetSocketLocation` (`self.Mesh`) "RightHandSocket") 100.0 12 (struct :`R` 1.0 :`G` 0.99351 :`A` 1.0) 0.0 1.0))

(fn `UserConstructionScript`
  (`parent.UserConstructionScript`))