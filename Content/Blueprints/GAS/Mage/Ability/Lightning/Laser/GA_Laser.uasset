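; Mage gameplay ability for a held-cast laser, aimed once at the point under the mouse on activation.
; It commits cost and cooldown, faces the avatar to the target, then plays a start montage that leads into a casting loop with movement disabled.
; Input release plays the end montage, whose completion or interruption restores movement and ends the ability.
; The laser montage event is awaited, but nothing handles it here.
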(event `self.K2_ActivateAbility`
  (if (`KismetSystemLibrary.DoesImplementInterface` (`self.GetAvatarActorFromActorInfo`) "/Script/ProjectGASRPG.CombatInterface")
    ;[1 1 1] cost && cooldown
    (`self.K2_CommitAbility`)
    (bind (_asynctaskproxy _targetdatahandle) (`TargetDataUnderMouse.CreateTargetDataUnderMouse`)
      (:`ValidData`
        (`self.StoreMouseDataInfo` (`AbilitySystemBlueprintLibrary.GetHitResultFromTargetData` _targetdatahandle))
        (message `CombatInterface.UpdateFacingTarget` (`self.GetAvatarActorFromActorInfo`) (`self.MouseHitLocation`))
        (`|ExecutionSequence`
          (:`then_0`
            (`AbilityTask_PlayMontageAndWait.CreatePlayMontageAndWaitProxy` "None" (`self.Montage Casting Start`) 1.0 "None" false
              (:`OnBlendOut`
                (message `CombatInterface.SetInCastingLoop` (`self.GetAvatarActorFromActorInfo`) true)
                (`self.Is Allow Move` false))))
          (:`then_1`
            ;[1 1 1] 等待Release事件
            (`AbilityTask_WaitInputRelease.WaitInputRelease` false
              (:`OnRelease`
                (message `CombatInterface.SetInCastingLoop` (`self.GetAvatarActorFromActorInfo`) false)
                (`AbilityTask_PlayMontageAndWait.CreatePlayMontageAndWaitProxy` "None" (`self.Montage Casting End`) 1.0 "None" false
                  (:`then`
                    (`AbilityTask_WaitGameplayEvent.WaitGameplayEvent` (struct :`TagName` "Event.Montage.Laser") null))
                  (:`OnCompleted`
                    (`self.Is Allow Move` true :!label _label)
                    (`self.K2_EndAbility`))
                  (:`OnBlendOut`
                    (goto _label))
                  (:`OnInterrupted`
                    (goto _label))
                  (:`OnCancelled`
                    (goto _label)))))))))
    (else
      (`self.K2_EndAbility`))))

(fn `Is Allow Move`
  (params (Allow :type Boolean))
  (if Allow
    ;[0 0 0] 开启移动
    (`CharacterMovementComponent.SetMovementMode` (`Character.CharacterMovement` (`GameplayStatics.GetPlayerCharacter` 0)) "MOVE_Walking" 0)
    (else
      ;[0 0 0] 禁止移动
      (`CharacterMovementComponent.DisableMovement` (`Character.CharacterMovement` (`GameplayStatics.GetPlayerCharacter` 0))))))