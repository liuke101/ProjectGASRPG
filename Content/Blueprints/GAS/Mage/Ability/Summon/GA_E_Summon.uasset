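; GA_E_Summon is a gameplay ability that summons randomly chosen pawns around the avatar.
; It shuffles the spawn locations, shows a ground Niagara effect at each, then plays the summon montage.
; A montage gameplay event starts a delayed loop that spawns each pawn with a default controller, facing along the summoner-to-spawn direction.
; Each spawn increments the avatar's summon count, and its OnDestroyed binding decrements it.
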(event `self.K2_ActivateAbility`
  (bind _output (`|GetArrayItem` (`self.SpawnLocations`) (`self.SpawnLocationIndex`)))
  (bind _output_get (set `self.SpawnLocations` (`self.GetSpawnLocations`)))
  ;[1 1 1] 增加随机性
  (`KismetArrayLibrary.Array_Shuffle` _output_get)
  (for _array_element _output_get
    (`NiagaraFunctionLibrary.SpawnSystemAtLocation` "/Game/Assets/Effects/Combat/NS_GroundSummon.NS_GroundSummon" _array_element))
  (`AbilityTask_PlayMontageAndWait.CreatePlayMontageAndWaitProxy` "None" "/Game/BlueProtocol/Enemy/E000/Anim/AM_E00_Summon.AM_E00_Summon"
    (:`then`
      ;[0.4637 0.861 1] 异步召唤
      (`AbilityTask_WaitGameplayEvent.WaitGameplayEvent` (struct :`TagName` "Montage.Attack.1") null
        (:`EventReceived`
          (if (< (`self.SpawnLocationIndex`) (`KismetArrayLibrary.Array_Length` (`self.SpawnLocations`))) :!label _label
            ;;[1 1 1] 运行时生成Pawn时，默认没有Controller，要手动生成
            (bind _returnvalue (`|SpawnActorFromClass` (`self.GetRandomSummonClass`) (`KismetMathLibrary.MakeTransform` _output (`KismetMathLibrary.FindLookAtRotation` (`Actor.K2_GetActorLocation` (`self.GetAvatarActorFromActorInfo`)) _output)) "Undefined" "MultiplyWithRoot" null null))
            (`Pawn.SpawnDefaultController` _returnvalue)
            ;;[1 1 1] 绑定召唤物死亡委托，数量-1
            (add `Actor.OnDestroyed` _returnvalue (delegate `OnDestroyed_Event`))
            ;;[1 1 1] 召唤物数量+1
            (message `CombatInterface.ModifySummonCount` (`self.GetAvatarActorFromActorInfo`) 1)
            (`/Engine/EditorBlueprintResources/StandardMacros.IncrementInt` (`self.SpawnLocationIndex`)
              (:`  `
                (`KismetSystemLibrary.Delay` 0.2)
                (goto _label)))))))))

(event `OnDestroyed_Event`
  (params (DestroyedActor :type "Actor Object Reference"))
  ;[0.4637 0.861 1] 异步召唤
  ;;[1 1 1] 绑定召唤物死亡委托，数量-1
  (message `CombatInterface.ModifySummonCount` (`self.GetAvatarActorFromActorInfo`) -1))