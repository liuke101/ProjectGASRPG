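; Mage fireball gameplay ability that launches a projectile at the location under the mouse cursor.
; On valid target data, it turns the avatar toward the target through CombatInterface and plays the cast montage.
; A custom anim notify sends the montage gameplay event that triggers SpawnProjectile.
; A short delay before EndAbility is a temporary workaround for server rollback when client prediction ends the ability before the projectile spawns.
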(event `self.K2_ActivateAbility`
  (bind (_asynctaskproxy _targetdatahandle) (`TargetDataUnderMouse.CreateTargetDataUnderMouse`)
    (:`ValidData`
      (set `self.TargetLocation` (`.Location` (`GameplayStatics.BreakHitResult` (`AbilitySystemBlueprintLibrary.GetHitResultFromTargetData` _targetdatahandle))))
      (bind _ascombat_interface (cast `CombatInterface` (`self.GetAvatarActorFromActorInfo`)))
      (`CombatInterface.UpdateFacingTarget` _ascombat_interface (`self.TargetLocation`))
      (`AbilityTask_PlayMontageAndWait.CreatePlayMontageAndWaitProxy` "None" "/Game/Anims/Mage/Animation/AM_Firaball.AM_Firaball"
        (:`then`
          ;[1 1 1] 由自定义的动画通知发送事件
          (`AbilityTask_WaitGameplayEvent.WaitGameplayEvent` (struct :`TagName` "Event.Montage.Fireball") null
            (:`EventReceived`
              (`self.SpawnProjectile` (`self.TargetLocation`))
              ;[1 1 1] 暂时使用delay处理，否则实际生成投射物之前的客户端预测阶段就调用EndAbility，服务器会回滚。
              (`KismetSystemLibrary.Delay` 0.2)
              (`self.K2_EndAbility`))))))))