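; Mage Fireball gameplay ability that casts a projectile toward the point under the mouse.
; On activation it commits cost and cooldown, gets cursor target data, turns the avatar toward that location and plays the fireball montage.
; A custom anim notify sends a gameplay event that triggers the projectile spawn from a tagged socket, syncing the shot to the animation.
; The ability ends when the montage completes, blends out, is interrupted or is cancelled.
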(event `self.K2_ActivateAbility`
  ;[1 1 1] cost && cooldown
  (`self.K2_CommitAbility`)
  (bind (_asynctaskproxy _targetdatahandle) (`TargetDataUnderMouse.CreateTargetDataUnderMouse`)
    (:`ValidData`
      (set `self.TargetLocation` (`.Location` (`GameplayStatics.BreakHitResult` (`AbilitySystemBlueprintLibrary.GetHitResultFromTargetData` _targetdatahandle))))
      (message `CombatInterface.UpdateFacingTarget` (`self.GetAvatarActorFromActorInfo`) (`self.TargetLocation`))
      (`AbilityTask_PlayMontageAndWait.CreatePlayMontageAndWaitProxy` "None" "/Game/Anims/Mage/Animation/AM_Firaball.AM_Firaball" (`self.AbilityMontageRate`) "None" false
        (:`then`
          ;[1 1 1] 由自定义的动画通知发送事件
          (`AbilityTask_WaitGameplayEvent.WaitGameplayEvent` (struct :`TagName` "Event.Montage.Fireball") null
            (:`EventReceived`
              (`self.SpawnProjectile` (`self.TargetLocation`) (`self.Socket Tag`)))))
        (:`OnCompleted`
          (`self.K2_EndAbility` :!label _label))
        (:`OnBlendOut`
          (goto _label))
        (:`OnInterrupted`
          (goto _label))
        (:`OnCancelled`
          (goto _label))))))