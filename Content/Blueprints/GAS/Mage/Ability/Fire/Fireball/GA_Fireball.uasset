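; Gameplay ability for the Mage's Fireball, which fires a projectile toward the location under the mouse.
; On activation it commits cost and cooldown, gets cursor target data, turns the avatar toward it and plays the cast montage.
; A custom anim notify's gameplay event triggers the projectile spawn, and the montage finishing or breaking off ends the ability.
; GetDescription builds rich-text Chinese tooltip text with level-based stats and a capped projectile count.
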(event `self.K2_ActivateAbility`
  ;[1 1 1] cost && cooldown
  (`self.K2_CommitAbility`)
  (bind (_asynctaskproxy _targetdatahandle) (`TargetDataUnderMouse.CreateTargetDataUnderMouse`)
    (:`ValidData`
      (set `self.TargetLocation` (`.Location` (`GameplayStatics.BreakHitResult` (`AbilitySystemBlueprintLibrary.GetHitResultFromTargetData` _targetdatahandle))))
      (message `CombatInterface.UpdateFacingTarget` (`self.GetAvatarActorFromActorInfo`) (`self.TargetLocation`))
      (`AbilityTask_PlayMontageAndWait.CreatePlayMontageAndWaitProxy` "None" "/Game/Anims/Mage/Animation/AM_Firaball.AM_Firaball" (`self.AbilityMontageRate`) "None" false
        (:`then`
          ;[1 1 1] 由自定义的动画通知发送事件
          (`AbilityTask_WaitGameplayEvent.WaitGameplayEvent` (struct :`TagName` "Event.Montage.Fireball") null
            (:`EventReceived`
              (`self.SpawnProjectile` (`self.TargetLocation`) (`self.Socket Tag`)))))
        (:`OnCompleted`
          (`self.K2_EndAbility` :!label _label))
        (:`OnBlendOut`
          (goto _label))
        (:`OnInterrupted`
          (goto _label))
        (:`OnCancelled`
          (goto _label))))))

(fn `GetDescription`
  (params (AbilityLevel :type Integer))
  (returns (ReturnValue :type String))
  (locals (Level :type Integer :default 0))
  (bind _level (`local.Level`))
  (set `local.Level` AbilityLevel)
  (return (`KismetTextLibrary.Conv_TextToString` (`|FormatText` "<Title>火球术</> \n<MainBody>技能等级：</><Level>{AbilityLevel}</> \n<MainBody>发射{ProjectileNum}个火球,有</><Damage>20%</><MainBody>几率点燃目标</> \n<MainBody>火属性伤害:</><Damage>{DamageValue}</> \n<MainBody>法力值消耗:</><Cost>{ManaCost}</> \n<MainBody>冷却时间:</><Cooldown>{Cooldown}s</>" (`local.Level`) (`KismetMathLibrary.Min` AbilityLevel (`self.MaxProjectileNum`)) (`self.GetTypeDamage` _level) (`self.GetManaCost` _level) (`self.GetCooldown` _level)))))