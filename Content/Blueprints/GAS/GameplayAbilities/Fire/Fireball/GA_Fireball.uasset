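; GA_Fireball is a Gameplay Ability that casts a fireball toward the location under the mouse cursor.
; On activation it waits for cursor target data, then turns the avatar toward the hit location through CombatInterface and plays a cast montage.
; A montage gameplay event times the projectile spawn at that target, after which the ability ends.
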(event `self.K2_ActivateAbility`
  (bind (_asynctaskproxy _targetdatahandle) (`TargetDataUnderMouse.CreateTargetDataUnderMouse`)
    (:`ValidData`
      (set `self.TargetLocation` (`.Location` (`GameplayStatics.BreakHitResult` (`AbilitySystemBlueprintLibrary.GetHitResultFromTargetData` _targetdatahandle))))
      (bind _ascombat_interface (cast `CombatInterface` (`self.GetAvatarActorFromActorInfo`)))
      (`CombatInterface.UpdateFacingTarget` _ascombat_interface (`self.TargetLocation`))
      (`AbilityTask_PlayMontageAndWait.CreatePlayMontageAndWaitProxy` "None" "/Game/Blueprints/Character/Anim/Montage/AM_TestMontage.AM_TestMontage"
        (:`then`
          (`AbilityTask_WaitGameplayEvent.WaitGameplayEvent` (struct :`TagName` "Event.Montage.Fireball") null
            (:`EventReceived`
              (`self.SpawnProjectile` (`self.TargetLocation`))
              (`self.K2_EndAbility`))))))))