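; Warrior melee gameplay ability that turns the avatar toward its combat target via motion warping and plays a spear attack montage.
; On the montage's melee event, it finds live players within a radius of the weapon socket, excluding the avatar, damages them and draws debug spheres.
; A short delay precedes EndAbility as a noted temporary workaround for server rollback when the ability ends during client prediction.
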(event `self.K2_ActivateAbility`
  (bind _avataractor (`self.AvatarActor`))
  ;[1 1 1] 获取战斗目标位置，调用MotionWarping面向敌人
  (bind _output_get (set `self.AvatarActor` (`self.GetAvatarActorFromActorInfo`)))
  (bind _ascombat_interface (cast `CombatInterface` _output_get))
  (bind _returnvalue (message `EnemyInterface.GetCombatTarget` (`self.AvatarActor`)))
  (`CombatInterface.UpdateFacingTarget` _ascombat_interface (`Actor.K2_GetActorLocation` _returnvalue))
  (`AbilityTask_PlayMontageAndWait.CreatePlayMontageAndWaitProxy` "None" "/Game/Blueprints/Enemy/Spear/Anim/AM_Spear_MeleeAtack.AM_Spear_MeleeAtack"
    (:`then`
      (`AbilityTask_WaitGameplayEvent.WaitGameplayEvent` (struct :`TagName` "Event.Montage.MeleeAttack") null
        (:`EventReceived`
          (bind _returnvalue_2 (message `CombatInterface.GetWeaponSocketLocation` (`self.AvatarActor`)))
          (bind _outoverlappingactors (`MageAbilitySystemLibrary.GetLivePlayerWithInRadius` _avataractor (`|MakeArray` _avataractor) _returnvalue_2 (`self.SphereRadius`)))
          (for _array_element _outoverlappingactors
            (`KismetSystemLibrary.DrawDebugSphere` (`Actor.K2_GetActorLocation` _array_element) 100.0 12 (struct :`R` 1.0 :`B` 0.620025 :`A` 1.0) 10.0 1.5)
            (`self.CauseDamage` _array_element))
          ;[1 1 1] 暂时使用delay处理，否则实际生成投射物之前的客户端预测阶段就调用EndAbility，服务器会回滚。
          (`KismetSystemLibrary.Delay` 0.2)
          (`self.K2_EndAbility`))))))