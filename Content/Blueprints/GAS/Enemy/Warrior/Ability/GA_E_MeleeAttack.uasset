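; Warrior enemy melee attack Gameplay Ability that turns toward its combat target and plays a random attack montage.
; A montage gameplay event triggers a sphere check at the weapon socket, damaging non-friendly live players in range and drawing debug spheres.
; On a hit it fires a MeleeAttack GameplayCue with the combat target as source object.
; The ability ends after that event or when the montage ends or is interrupted.
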(event `self.K2_ActivateAbility`
  (bind _avataractor (`self.AvatarActor`))
  (set `self.bHasHitTarget` false)
  (`|ExecutionSequence`
    (:`then_0`
      ;[1 1 1] 获取战斗目标位置，调用MotionWarping面向敌人
      (bind _output_get (set `self.AvatarActor` (`self.GetAvatarActorFromActorInfo`)))
      (bind _returnvalue (message `EnemyInterface.GetCombatTarget` _output_get))
      (bind _output_get_2 (set `self.CombatTarget` _returnvalue))
      (message `CombatInterface.UpdateFacingTarget` _output_get_2 (`Actor.K2_GetActorLocation` _returnvalue)))
    (:`then_1`
      ;[1 1 1] 获取Attack蒙太奇（从数组中随机选一个）
      (bind _returnvalue_2 (message `CombatInterface.GetRandomAttackMontage` (`self.AvatarActor`)))
      (bind _output_get_3 (set `self.TaggedMontage` _returnvalue_2))
      (bind (_montage _montagetag _sockettag _impactsound) (break `TaggedMontage` _output_get_3))
      ;;[1 1 1] Montage和Tag对应
      (set `self.Montage` _montage)
      (set `self.Montage Tag` _montagetag)
      (set `self.Socket Tag` _sockettag)
      (set `self.Impact Sound` _impactsound))
    (:`then_2`
      ;[1 0.6046 0.5827] Ability Task
      (`AbilityTask_PlayMontageAndWait.CreatePlayMontageAndWaitProxy` "None" (`self.Montage`) 1.0 "None" false
        (:`then`
          ;;[1 1 1] 等待由蒙太奇发起的通知
          (`AbilityTask_WaitGameplayEvent.WaitGameplayEvent` (`self.Montage Tag`) null
            (:`EventReceived`
              ;;[1 1 1] 获取Socket为圆心的球体体积的玩家
              (bind _returnvalue_3 (message `CombatInterface.GetWeaponSocketLocationByTag` (`self.AvatarActor`) (`self.Socket Tag`)))
              (bind _output_get_4 (set `self.WeaponSocketLocation` _returnvalue_3))
              (`KismetSystemLibrary.DrawDebugSphere` (`self.WeaponSocketLocation`) (`self.SphereRadius`) 12 (struct :`R` 1.0 :`G` 0.021999 :`A` 1.0) 1.0 1.0)
              (bind _outoverlappingactors (`MageAbilitySystemLibrary.GetLivePlayerWithInRadius` _avataractor (`|MakeArray` _avataractor) _output_get_4 (`self.SphereRadius`)))
              ;;[1 1 1] 如果不是友方，就造成伤害
              (for _array_element _outoverlappingactors
                (if (not (`MageAbilitySystemLibrary.IsFriendly` (`self.AvatarActor`) _array_element))
                  (`KismetSystemLibrary.DrawDebugSphere` (`Actor.K2_GetActorLocation` _array_element) 100.0 12 (struct :`R` 1.0 :`B` 0.620025 :`A` 1.0) 10.0 1.5)
                  (`self.CauseDamage` _array_element)
                  (set `self.bHasHitTarget` true)))
              (if (`self.bHasHitTarget`)
                ;;[1 0.4179 0.9123] GameplayCue
                (`self.K2_ExecuteGameplayCueWithParams` (struct :`TagName` "GameplayCue.MeleeAttack") (`AbilitySystemBlueprintLibrary.MakeGameplayCueParameters` 0.0 0.0 (struct) (struct) (struct) (`BlueprintGameplayTagLibrary.MakeGameplayTagContainerFromTag` (`.MontageTag` (break `TaggedMontage` (`self.TaggedMontage`)))) (struct) (`self.WeaponSocketLocation`) (0.0 0.0 0.0) null (`self.AvatarActor`) (`self.CombatTarget`))))
              (`self.K2_EndAbility`))))
        (:`OnCompleted`
          ;;[1 1 1] 防止上面的流程被打断导致无法End
          (`self.K2_EndAbility` :!label _label))
        (:`OnBlendOut`
          (goto _label))
        (:`OnInterrupted`
          (goto _label))
        (:`OnCancelled`
          (goto _label))))))