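; Enemy ranged-attack gameplay ability that turns toward the combat target and fires a projectile at it.
; It caches the target's location, updates motion-warp facing, then picks a random attack montage with its event tag and socket tag.
; The montage's gameplay event triggers SpawnProjectile once, aimed at the cached location with optional pitch override.
; The ability ends when the montage completes, blends out, is interrupted or is cancelled.
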(event `self.K2_ActivateAbility`
  (`|ExecutionSequence`
    (:`then_0`
      ;[1 1 1] 获取战斗目标位置，调用MotionWarping面向敌人
      (bind _output_get (set `self.AvatarActor` (`self.GetAvatarActorFromActorInfo`)))
      (bind _returnvalue (message `EnemyInterface.GetCombatTarget` _output_get))
      (bind _output_get_2 (set `self.TargetLocation` (`Actor.K2_GetActorLocation` _returnvalue)))
      (message `CombatInterface.UpdateFacingTarget` _returnvalue _output_get_2))
    (:`then_1`
      ;[1 1 1] 获取Attack蒙太奇（从数组中随机选一个）
      (bind _returnvalue_2 (message `CombatInterface.GetRandomAttackMontage` (`self.AvatarActor`)))
      (bind _output_get_3 (set `self.TaggedMontage` _returnvalue_2))
      (bind (_montage _montagetag _sockettag) (break `TaggedMontage` _output_get_3))
      ;;[1 1 1] Montage和Tag对应
      (set `self.Montage` _montage)
      (set `self.Montage Tag` _montagetag)
      (set `self.Socket Tag` _sockettag))
    (:`then_2`
      ;[1 0.7037 0.7537] AbilityTask
      (`AbilityTask_PlayMontageAndWait.CreatePlayMontageAndWaitProxy` "None" (`self.Montage`) 1.0 "None" false
        (:`then`
          ;;[1 1 1] 等待由蒙太奇发起的通知
          (`AbilityTask_WaitGameplayEvent.WaitGameplayEvent` (`self.Montage Tag`) null true
            (:`EventReceived`
              (`self.SpawnProjectile` (`self.TargetLocation`) (`self.Socket Tag`) (`self.bOverride Pitch`) (`self.Pitch Override`)))))
        (:`OnCompleted`
          ;;[1 1 1] 防止上面的流程被打断导致无法End
          (`self.K2_EndAbility` :!label _label))
        (:`OnBlendOut`
          (goto _label))
        (:`OnInterrupted`
          (goto _label))
        (:`OnCancelled`
          (goto _label))))))