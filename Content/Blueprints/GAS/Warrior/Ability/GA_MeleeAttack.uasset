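; GA_MeleeAttack is a Warrior Gameplay Ability that performs a melee attack against nearby enemies.
; It turns the avatar toward its combat target for motion warping, then plays a random tagged attack montage.
; The montage's gameplay event triggers a radius query at the weapon socket, damaging live non-friendly actors and drawing debug spheres.
; A short delay before ending works around prediction rollback; montage completion, blend-out or interruption also ends it.
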(event `self.K2_ActivateAbility`
  (bind _avataractor (`self.AvatarActor`))
  (`|ExecutionSequence`
    (:`then_0`
      ;[1 1 1] 获取战斗目标位置，调用MotionWarping面向敌人
      (bind _output_get (set `self.AvatarActor` (`self.GetAvatarActorFromActorInfo`)))
      (bind _ascombat_interface (cast `CombatInterface` _output_get))
      (bind _returnvalue (message `EnemyInterface.GetCombatTarget` (`self.AvatarActor`)))
      (`CombatInterface.UpdateFacingTarget` _ascombat_interface (`Actor.K2_GetActorLocation` _returnvalue)))
    (:`then_1`
      ;[1 1 1] 获取Attack蒙太奇（从数组中随机选一个）
      (bind _returnvalue_2 (message `CombatInterface.GetAttackMontages` (`self.AvatarActor`)))
      (if (`KismetArrayLibrary.Array_IsEmpty` _returnvalue_2)
        (`self.K2_EndAbility`)
        (else
          (bind _output_get_2 (set `self.TaggedMontage` (`KismetArrayLibrary.Array_Random` _returnvalue_2)))
          (bind (_montage _montagetag) (break `TaggedMontage` _output_get_2))
          ;[1 1 1] Montage和Tag对应
          (set `self.Montage` _montage)
          (set `self.Montage Tag` _montagetag)
          (`AbilityTask_PlayMontageAndWait.CreatePlayMontageAndWaitProxy` "None" (`self.Montage`) 1.0 "None" false
            (:`then`
              ;[1 1 1] 等待由蒙太奇发起的通知
              (`AbilityTask_WaitGameplayEvent.WaitGameplayEvent` (`self.Montage Tag`) null
                (:`EventReceived`
                  (bind _returnvalue_3 (message `CombatInterface.GetWeaponSocketLocation` (`self.AvatarActor`) (`self.Montage Tag`)))
                  (bind _outoverlappingactors (`MageAbilitySystemLibrary.GetLivePlayerWithInRadius` _avataractor (`|MakeArray` _avataractor) _returnvalue_3 (`self.SphereRadius`)))
                  (for _array_element _outoverlappingactors
                    (if (not (`MageAbilitySystemLibrary.IsFriendly` (`self.AvatarActor`) _array_element))
                      (`KismetSystemLibrary.DrawDebugSphere` (`Actor.K2_GetActorLocation` _array_element) 100.0 12 (struct :`R` 1.0 :`B` 0.620025 :`A` 1.0) 10.0 1.5)
                      (`self.CauseDamage` _array_element)))
                  ;[1 1 1] 暂时使用delay处理，否则实际生成投射物之前的客户端预测阶段就调用EndAbility，服务器会回滚。
                  (`KismetSystemLibrary.Delay` 0.2)
                  (`self.K2_EndAbility`))))
            (:`OnCompleted`
              ;[1 1 1] 防止上面的流程被打断导致无法End
              (`self.K2_EndAbility` :!label _label))
            (:`OnBlendOut`
              (goto _label))
            (:`OnInterrupted`
              (goto _label))
            (:`OnCancelled`
              (goto _label))))))))