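; GA_Dash is a player gameplay ability that provides a hold-to-dash, raising move speed while input is held.
; On activation it applies the GE_MoveSpeedUp effect, adds the Dash gameplay cue and starts a looping timer that commits the ability cost.
; Input release or a failed cost commit calls RemoveAbility, which clears the timer, removes the effect and cue, and ends the ability.
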(event `self.K2_ActivateAbility`
  (bind _returnvalue (`self.BP_ApplyGameplayEffectToOwner` "/Game/Blueprints/GAS/Common/Effect/DefaultAttributes/GE_MoveSpeedUp.GE_MoveSpeedUp_C"))
  (set `self.GE Handle` _returnvalue)
  (`AbilityTask_WaitInputRelease.WaitInputRelease` false
    (:`then`
      (bind _output_get (set `self.GC Params` (`AbilitySystemBlueprintLibrary.MakeGameplayCueParameters` 0.0)))
      (`GameplayCueFunctionLibrary.AddGameplayCueOnActor` (`self.GetAvatarActorFromActorInfo`) (struct :`TagName` "GameplayCue.Dash") _output_get)
      (bind _returnvalue_2 (`KismetSystemLibrary.K2_SetTimerDelegate` (delegate `CommitCost_Event`) (`self.Delta Cost Time`) true))
      (set `self.Timer Handle` _returnvalue_2))
    (:`OnRelease`
      (`self.Remove Ability`))))

(event `CommitCost_Event`
  (bind _returnvalue (`self.K2_CommitAbilityCost` false))
  (if (not _returnvalue)
    (`self.Remove Ability`)))

(fn `Remove Ability`
  (locals (NewLocalVar :type "Actor Object Reference"))
  (`KismetSystemLibrary.K2_ClearAndInvalidateTimerHandle` (`self.Timer Handle`))
  (`self.BP_RemoveGameplayEffectFromOwnerWithHandle` (`self.GE Handle`))
  (`GameplayCueFunctionLibrary.RemoveGameplayCueOnActor` (`self.GetAvatarActorFromActorInfo`) (struct :`TagName` "GameplayCue.Dash") (`self.GC Params`))
  (`self.K2_EndAbility`))