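; Passive player ability that turns incoming gameplay events under the Attribute tag into attribute changes on its owner.
; On activation it waits for matching events, including child tags, and builds a spec from EventBasedEffectClass.
; It loops over EventTags, setting the SetByCaller magnitude to the event's value for the exact match and zero for the rest, avoiding unset-magnitude errors.
; It then applies the spec to its own ASC.
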(event `self.K2_ActivateAbility`
  (bind _returnvalue (`self.GetAbilitySystemComponentFromActorInfo`))
  ;[1 1 1] 一般由SendGameplayEventToActor函数发送Tag事件并传来payload
  (bind (_asynctaskproxy _payload) (`AbilityTask_WaitGameplayEvent.WaitGameplayEvent` (struct :`TagName` "Attribute") null false false)
    (:`EventReceived`
      (bind (_eventtag _instigator _target _optionalobject _optionalobject2 _contexthandle _instigatortags _targettags _eventmagnitude) (break `GameplayEventData` _payload))
      ;[0.7348 0.7544 1] SetByCaller GE, 将EventMagnitude传给Tag对应的属性
      (set `self.Event Tag` _eventtag)
      (set `self.Event Magnitude` _eventmagnitude)
      (set `self.GE Spec Handle` (`AbilitySystemComponent.MakeOutgoingSpec` _returnvalue (`self.EventBasedEffectClass`) 1.0 (`AbilitySystemComponent.MakeEffectContext` _returnvalue)))
      ;;[1 0.6448 0.6448] 遍历EventTags数组，如果传进来的EventTag和数组中的元素匹配，则设置对应的Magenitude。不匹配则设为0（必须为GE中每一个使用SetByCaller的Modifier 分配Magnitude值，并将返回的SpecHandle应用，否则会报错 FGameplayEffectSpec::GetMagnitude called for Data Attribute.XXX.XXX on Def Default__GE_EventBaseEffect_C when magnitude had not yet been set by caller.）
      (for _array_element (`self.EventTags`)
        (if (`BlueprintGameplayTagLibrary.MatchesTag` _array_element (`self.Event Tag`) true)
          (`AbilitySystemBlueprintLibrary.AssignTagSetByCallerMagnitude` (`self.GE Spec Handle`) (`self.Event Tag`) (`self.Event Magnitude`))
          (else
            (`AbilitySystemBlueprintLibrary.AssignTagSetByCallerMagnitude` (`self.GE Spec Handle`) _array_element))))
      (`AbilitySystemComponent.BP_ApplyGameplayEffectSpecToSelf` (`self.GetAbilitySystemComponentFromActorInfo`) (`self.GE Spec Handle`)))))