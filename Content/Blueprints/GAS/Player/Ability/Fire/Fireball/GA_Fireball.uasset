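; GA_Fireball is the player's Fireball gameplay ability, launching a level-scaled number of homing fire projectiles at a target.
; On activation it commits cost and cooldown, faces the target and plays the cast montage.
; A montage gameplay event triggers the projectile spawn, and any montage exit ends the ability.
; GetDescription builds Chinese rich-text skill info from level-based count, damage, cost and cooldown, plus ignite chance.
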(event `self.K2_ActivateAbility`
  ;[1 0.8906 0] cost && cooldown
  (`self.K2_CommitAbility`)
  (`self.GetTargetingActorInfo`)
  (message `CombatInterface.UpdateFacingTarget` (`self.GetAvatarActorFromActorInfo`) (`self.TargetingActorLocation`))
  (`AbilityTask_PlayMontageAndWaitForGameplayEvent.PlayMontageAndWaitForGameplayEvent` "None" "/Game/Anims/Mage/Animation/AM_Fireball.AM_Fireball" (struct :`GameplayTags` (struct :`(TagName` "Event.Montage.Fireball"))) (`self.AbilityMontageRate`) "None" false
    (:`OnCompleted`
      (`self.K2_EndAbility` :!label _label))
    (:`OnBlendOut`
      (goto _label))
    (:`OnInterrupted`
      (goto _label))
    (:`OnCancelled`
      (goto _label))
    (:`EventReceived`
      (`self.SpawnMultiProjectiles` (`self.TargetingActor`) (`self.TargetingActorLocation`) (`self.GetSpawnProjectilesNum` (`self.GetAbilityLevel`)) (`self.Attack Socket Tag`) true))))

(fn `GetDescription`
  (params (AbilityLevel :type Integer))
  (returns (ReturnValue :type String))
  (locals (Level :type Integer :default 0))
  (bind _level (`local.Level`))
  (set `local.Level` AbilityLevel)
  (return (`KismetTextLibrary.Conv_TextToString` (`|FormatText` "<Title>火球术</> \n<MainBody>技能等级：</><Level>{AbilityLevel}</> \n<MainBody>发射{ProjectileNum}个火球,有</><Damage>{DebuffChance}%</><MainBody>几率点燃目标</> \n<MainBody>火属性伤害:</><Damage>{DamageValue}</> \n<MainBody>法力值消耗:</><Cost>{ManaCost}</> \n<MainBody>冷却时间:</><Cooldown>{Cooldown}s</>" (`local.Level`) (`self.GetSpawnProjectilesNum` (`local.Level`)) (* (`self.DebuffChance`) 100.0) (`self.GetTypeDamage` _level) (`self.GetManaCost` _level) (`self.GetCooldown` _level)))))