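; GA_IceBlast is a player ice ability that deals two waves of area damage at a magic circle.
; The circle shows on activation; releasing input commits, hides it and plays the montage.
; The montage event fires the GameplayCue immediately, then delayed capsule and wider sphere overlaps apply default damage to living actors except the caster.
; The ability ends after the second wave or on montage interruption or cancellation.
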(event `self.K2_ActivateAbility`
  (message `PlayerInterface.ShowMagicCircle` (`self.GetAvatarActorFromActorInfo`) null)
  (`AbilityTask_WaitInputRelease.WaitInputRelease` false
    (:`OnRelease`
      (`self.K2_CommitAbility`)
      (message `PlayerInterface.HideMagicCircle` (`self.GetAvatarActorFromActorInfo`))
      (`MageAT_PlayMontageAndWaitForGameplayEvent.PlayMontageAndWaitForGameplayEvent` "None" "/Game/Anims/Mage/Animation/AM_IceBlast.AM_IceBlast" (struct :`GameplayTags` (struct :`(TagName` "Event.Montage.IceBlast")))
        (:`OnInterrupted`
          (`self.K2_EndAbility` :!label _label))
        (:`OnCancelled`
          (goto _label))
        (:`EventReceived`
          (`GameplayTask_WaitDelay.TaskWaitDelay` null 2.0
            (:`then`
              ;[1 0.002502 0.7689] GameplayCue
              (`self.K2_ExecuteGameplayCueWithParams` (struct :`TagName` "GameplayCue.IceBlast") (`AbilitySystemBlueprintLibrary.MakeGameplayCueParameters` 0.0 0.0 (struct) (struct) (struct) (struct) (struct) (- (`MageAbilitySystemLibrary.GetMagicCircleLocation` null) (300.0 0.0 0.0)))))
            (:`OnFinish`
              ;[1 0.03136 0] 第一段伤害
              (bind _outoverlappingactors (`MageAbilitySystemLibrary.GetLivingActorInCollisionShape` null (`|MakeArray` (`self.GetAvatarActorFromActorInfo`)) (`MageAbilitySystemLibrary.GetMagicCircleLocation` null) "Capsule" true 0.0 (200.0 200.0 200.0) 400.0 800.0))
              (for _array_element _outoverlappingactors
                (`MageAbilitySystemLibrary.ApplyDamageEffect` (`self.MakeDamageEffectParamsFromClassDefault` _array_element)))
              (`GameplayTask_WaitDelay.TaskWaitDelay` null 3.5
                (:`OnFinish`
                  ;[1 0.02436 0.05818] 第二段伤害
                  (bind _outoverlappingactors_2 (`MageAbilitySystemLibrary.GetLivingActorInCollisionShape` null (`|MakeArray` (`self.GetAvatarActorFromActorInfo`)) (`MageAbilitySystemLibrary.GetMagicCircleLocation` null) "Sphere" true 700.0))
                  (for _array_element_2 _outoverlappingactors_2
                    (`MageAbilitySystemLibrary.ApplyDamageEffect` (`self.MakeDamageEffectParamsFromClassDefault` _array_element_2)))
                  (`self.K2_EndAbility`))))))))))