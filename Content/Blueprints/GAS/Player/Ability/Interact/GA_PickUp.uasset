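; GA_PickUp is a Gameplay Ability that lets the avatar pick up the nearest MageItem.
; It plays AM_PickUp and, on the montage's Event.PickUp event, gathers MageItems in a debug-drawn capsule around the avatar and selects the closest.
; That item goes to the overlay widget controller for pickup display and to the avatar's inventory component.
; The ability ends when the montage completes, blends out, is interrupted or is cancelled.
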(event `self.K2_ActivateAbility`
  (bind _returnvalue (`Actor.K2_GetActorLocation` (`self.GetAvatarActorFromActorInfo`)))
  (`MageAT_PlayMontageAndWaitForGameplayEvent.PlayMontageAndWaitForGameplayEvent` "None" "/Game/Anims/Mage/Animation/AM_PickUp.AM_PickUp" (struct :`GameplayTags` (struct :`(TagName` "Event.PickUp")))
    (:`OnCompleted`
      (`self.K2_EndAbility` :!label _label))
    (:`OnBlendOut`
      (goto _label))
    (:`OnInterrupted`
      (goto _label))
    (:`OnCancelled`
      (goto _label))
    (:`EventReceived`
      ;[1 1 1] 获取范围内最近的Item
      (bind _outoverlappingactors (`MageAbilitySystemLibrary.GetActorInCollisionShapeWithClass` null "/Script/ProjectGASRPG.MageItem" (`|MakeArray` null :!type "Actor Object Reference") _returnvalue "Capsule" true 0.0 (0.0 0.0 0.0) 70.0 100.0))
      (bind _returnvalue_2 (`MageAbilitySystemLibrary.GetClosestActor` _outoverlappingactors _returnvalue))
      (bind _asmage_item (cast `MageItem` _returnvalue_2))
      ;[1 1 1] OverlayWidget监听拾取信息
      (bind _output_get (set `self.Mage Item` _asmage_item))
      (`MageWidgetController.SetMageItem` (`MageAbilitySystemLibrary.GetOverlayWidgetController` null) _output_get)
      ;[1 1 1] 库存系统增加Item
      (bind _returnvalue_3 (message `PlayerInterface.GetInventoryComponent` (`self.GetAvatarActorFromActorInfo`)))
      (`InventoryComponent.AddItem` _returnvalue_3 (`self.Mage Item`)))))