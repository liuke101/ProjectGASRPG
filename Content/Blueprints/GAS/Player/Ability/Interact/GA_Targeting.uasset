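; GA_Targeting is a player Gameplay Ability that runs ground-trace targeting with a world reticle and reports what was hit.
; On activation it starts a WaitTargetData task with debug drawing, tracing from the targeting actor supplied by BP_MagePlayerController and showing BP_TargetReticle.
; Confirmation is set to Custom, and valid data only prints the hit actor's name.
; The graph never ends the ability or handles cancellation.
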(event `self.K2_ActivateAbility`
  (bind _asbp_mage_player_controller (cast `/Game/Blueprints/Character/BP_MagePlayerController` (`GameplayStatics.GetPlayerController` 0)))
  (bind (_asynctaskproxy _data) (`AbilityTask_WaitTargetData.WaitTargetData` "123" "Custom" "/Script/GameplayAbilities.GameplayAbilityTargetActor_GroundTrace" 10.0 0.0 999999.0 (struct :`Name` "BlockAllDynamic") false (make `GameplayAbilityTargetingLocationInfo` "ActorTransform" "0.000000,0.000000,0.000000|0.000000,0.000000,-0.000000|1.000000,1.000000,1.000000" (`MagePlayerController.GetTargetingActor` _asbp_mage_player_controller) null self) (make `WorldReticleParameters` (1.0 1.0 1.0)) "/Game/Blueprints/GAS/Player/Ability/Interact/BP_TargetReticle.BP_TargetReticle_C" (struct) true)
    (:`ValidData`
      (`KismetSystemLibrary.PrintString` (`KismetSystemLibrary.GetDisplayName` (`.HitActor` (`GameplayStatics.BreakHitResult` (`AbilitySystemBlueprintLibrary.GetHitResultFromTargetData` _data))))))))