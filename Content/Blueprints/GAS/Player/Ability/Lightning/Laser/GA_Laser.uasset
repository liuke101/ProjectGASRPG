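; GA_Laser is a player Gameplay Ability that fires a charged lightning laser at the mouse target.
; On release, hold time sets the damage tier and a montage event starts Gameplay Cue beams, chaining from an enemy to nearby targets capped by ability level.
; A looping timer commits cost and damages enemies, or only drains cost on non-enemy hits.
; Montage end or failed cost clears the cues and applies a final damage effect to enemies.
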(event `self.K2_ActivateAbility`
  ;[0 0 0] 预处理
  (bind _output_get (set `self.Avatar Actor` (`self.GetAvatarActorFromActorInfo`)))
  (if (`KismetSystemLibrary.DoesImplementInterface` _output_get "/Script/ProjectGASRPG.CombatInterface")
    (bind (_asynctaskproxy _targetdatahandle) (`TargetDataUnderMouse.CreateTargetDataUnderMouse`)
      (:`ValidData`
        (`self.StoreMouseDataInfo` (`AbilitySystemBlueprintLibrary.GetHitResultFromTargetData` _targetdatahandle))
        (message `CombatInterface.UpdateFacingTarget` (`self.Avatar Actor`) (`self.MouseHitLocation`))
        (`|ExecutionSequence`
          (:`then_0`
            (`AbilityTask_PlayMontageAndWait.CreatePlayMontageAndWaitProxy` "None" (`self.Montage Casting Start`)
              (:`OnBlendOut`
                ;[1 1 1] 将动画蓝图状态切换到Casting Loop
                (message `CombatInterface.SetInCastingLoop` (`self.Avatar Actor`) true))))
          (:`then_1`
            ;[1 1 1] 等待Release事件
            (bind (_asynctaskproxy_2 _timeheld) (`AbilityTask_WaitInputRelease.WaitInputRelease` false)
              (:`OnRelease`
                (set `self.Time Held` _timeheld)
                (message `CombatInterface.SetInCastingLoop` (`self.Avatar Actor`) false)
                (`AbilityTask_PlayMontageAndWait.CreatePlayMontageAndWaitProxy` "None" (`self.Montage Casting End`)
                  (:`then`
                    (`AbilityTask_WaitGameplayEvent.WaitGameplayEvent` (struct :`TagName` "Event.Montage.Laser") null
                      (:`EventReceived`
                        ;[0 0.001522 1] Gameplay Cue
                        (`self.Add GC`
                          (:`Target Is Enemy `
                            ;[1 0.9618 0.9805] 命中敌人，计算Damage和Cost
                            (bind _returnvalue (`KismetSystemLibrary.K2_SetTimerDelegate` (delegate `DamageAndCost`) (`self.DamageDeltaTime`) true))
                            (set `self.Damage And Cost Timer` _returnvalue))
                          (:`Target Is  Common Actor`
                            ;[1 1 1] 没有命中敌人，只需要计算Cost
                            (bind _returnvalue_2 (`KismetSystemLibrary.K2_SetTimerDelegate` (delegate `OnlyCost`) (`self.DamageDeltaTime`) true))
                            (set `self.Only Cost Timer` _returnvalue_2))))))
                  (:`OnCompleted`
                    (`self.K2_EndAbility` :!label _label)
                    (`self.Remove All GC`)
                    ;[0.3739 1 0.8574] Cooldown
                    (`self.K2_CommitAbilityCooldown` false))
                  (:`OnBlendOut`
                    (goto _label))
                  (:`OnInterrupted`
                    (goto _label))
                  (:`OnCancelled`
                    (goto _label)))))))))
    (else
      (`self.K2_EndAbility`))))

(event `DamageAndCost`
  ;[1 0.9618 0.9805] 命中敌人，计算Damage和Cost
  ;;[0 0.9871 1] Cost
  (bind _returnvalue (`self.K2_CommitAbilityCost` false))
  (if _returnvalue
    ;;[1 0 0.01207] Damage
    (`self.Apply Damage`)
    (else
      (`KismetSystemLibrary.K2_ClearAndInvalidateTimerHandle` (`self.Damage And Cost Timer`))
      (`self.K2_EndAbility`)
      (`self.Remove All GC`))))

(event `self.OnTargetDiedCallback`
  (params (DeadActor :type "Actor Object Reference"))
  ;[1 1 1] OnTargetDied委托回调，移除死亡Actor对应的GC
  (`GameplayCueFunctionLibrary.RemoveGameplayCueOnActor` DeadActor (struct :`TagName` "GameplayCue.CastingLoop") (`self.First Target GC Params`)))

(event `OnlyCost`
  ;[1 1 1] 没有命中敌人，只需要计算Cost
  ;;[0 0.9871 1] Cost
  (bind _returnvalue (`self.K2_CommitAbilityCost` false))
  (if (not _returnvalue)
    (`KismetSystemLibrary.K2_ClearAndInvalidateTimerHandle` (`self.Only Cost Timer`))
    (`self.K2_EndAbility`)
    (`self.Remove All GC`)))

(fn `Add  GC To Additional Target`
  (params (`Additional Target` :type "Actor Object Reference"))
  (locals (TargetActor :type "Actor Object Reference"))
  (bind _targetactor (`local.TargetActor`))
  (bind _returnvalue (`AbilitySystemBlueprintLibrary.MakeGameplayCueParameters` 0.0 (`self.Time Held`) (struct) (struct) (struct) (struct) (struct) (`Actor.K2_GetActorLocation` _targetactor) (0.0 0.0 0.0) null null _targetactor null 1 1 (`Actor.RootComponent` (`self.MouseHitActor`))))
  (set `local.TargetActor` `Additional Target`)
  ;[1 1 1] 构建Map
  (`BlueprintMapLibrary.Map_Add` (`self.Additional Actors_To_GC Params`) (`local.TargetActor`) _returnvalue)
  (`GameplayCueFunctionLibrary.AddGameplayCueOnActor` (`local.TargetActor`) (struct :`TagName` "GameplayCue.CastingLoop") _returnvalue))

(fn `Apply Damage`
  (bind _additional_targets (`self.Additional Targets`))
  (`self.Apply Damge Single Target` (`self.MouseHitActor`))
  (if (not (`KismetArrayLibrary.Array_IsEmpty` _additional_targets))
    (for _array_element _additional_targets
      (`self.Apply Damge Single Target` _array_element))))

(fn `Apply Damge Single Target`
  (params (Actor :type "Actor Object Reference"))
  (locals (TargetASC :type "AbilitySystemComponent Object Reference"))
  (bind _returnvalue (`self.GetAbilitySystemComponentFromActorInfo`))
  (bind _returnvalue_2 (`self.GetAbilityLevel`))
  (set `local.TargetASC` (`AbilitySystemBlueprintLibrary.GetAbilitySystemComponent` Actor))
  (bind _returnvalue_3 (`AbilitySystemBlueprintLibrary.AssignTagSetByCallerMagnitude` (`AbilitySystemComponent.MakeOutgoingSpec` _returnvalue (`self.DamageEffectClass`) (`KismetMathLibrary.Conv_IntToDouble` _returnvalue_2) (`AbilitySystemComponent.MakeEffectContext` _returnvalue)) (struct :`TagName` "DamageType.Lightning") (`self.GetDamageByTimeHeld` (`self.Time Held`) (`self.GetTypeDamage` _returnvalue_2))))
  (`AbilitySystemComponent.BP_ApplyGameplayEffectSpecToSelf` (`local.TargetASC`) _returnvalue_3))

(fn `GetDamageByTimeHeld`
  (params (TimeHeld :type "Float (single-precision)") (TypeDamage :type "Float (double-precision)"))
  (returns (Damage :type "Float (double-precision)"))
  (locals (DamageValue :type "Float (double-precision)"))
  (set `local.DamageValue` TypeDamage)
  (`MageAbilitySystemLibrary.GetAbilityLayerByTimeHeld` TimeHeld
    (:`Layer1`
      (set `local.DamageValue` (* (`local.DamageValue`) 1.0)))
    (:`Layer2`
      (set `local.DamageValue` (* (`local.DamageValue`) 2.0)))
    (:`Layer3`
      (set `local.DamageValue` (* (`local.DamageValue`) 3.0)))
    (:`Layer4`
      (set `local.DamageValue` (* (`local.DamageValue`) 4.0))))
  (return (`local.DamageValue`)))

(fn `Remove All GC`
  (if (`self.First Target Is Combat Interface`)
    ;[1 1 1] 移除第一目标敌人的GC
    (`GameplayCueFunctionLibrary.RemoveGameplayCueOnActor` (`self.MouseHitActor`) (struct :`TagName` "GameplayCue.CastingLoop") (`self.First Target GC Params`))
    ;[1 1 1] 只在最后应用一个Debuff
    (`MageAbilitySystemLibrary.ApplyDamageEffect` (`self.MakeDamageEffectParamsFromClassDefault` (`self.MouseHitActor`)))
    ;[1 1 1] 移除其他目标敌人的GC
    (for _array_element (`self.Additional Targets`)
      (bind (_value _returnvalue) (`BlueprintMapLibrary.Map_Find` (`self.Additional Actors_To_GC Params`) _array_element))
      (if _returnvalue
        (`GameplayCueFunctionLibrary.RemoveGameplayCueOnActor` _array_element (struct :`TagName` "GameplayCue.CastingLoop") _value)
        (`MageAbilitySystemLibrary.ApplyDamageEffect` (`self.MakeDamageEffectParamsFromClassDefault` _array_element))))
    (else
      ;[1 1 1] 移除自身的GC
      (`GameplayCueFunctionLibrary.RemoveGameplayCueOnActor` (`self.Avatar Actor`) (struct :`TagName` "GameplayCue.CastingLoop") (`self.First Target GC Params`)))))