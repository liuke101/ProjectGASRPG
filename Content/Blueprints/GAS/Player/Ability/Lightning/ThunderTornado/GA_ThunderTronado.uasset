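; Gameplay ability for the player's Thunder Tornado spell, aimed with a magic circle while input is held.
; On release it commits, plays the cast montage and, on its gameplay event, starts the tornado cue at the circle.
; Living enemies in a wide capsule get radial root-motion force, while a delayed, narrower capsule query applies damage.
; Cue removal and normal ability end hang off each affected enemy's duration wait.
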(event `self.K2_ActivateAbility`
  (bind _returnvalue (`self.GetAvatarActorFromActorInfo`))
  (message `PlayerInterface.ShowMagicCircle` (`self.GetAvatarActorFromActorInfo`) null)
  (`AbilityTask_WaitInputRelease.WaitInputRelease` false
    (:`OnRelease`
      (`self.K2_CommitAbility`)
      (message `PlayerInterface.HideMagicCircle` (`self.GetAvatarActorFromActorInfo`))
      (`MageAT_PlayMontageAndWaitForGameplayEvent.PlayMontageAndWaitForGameplayEvent` "None" "/Game/Anims/Mage/Animation/AM_ThunderTronado.AM_ThunderTronado" (struct :`GameplayTags` (struct :`(TagName` "Event.Montage.IceBlast") :`(TagName` "Event.Montage.ThunderTronado")))
        (:`OnInterrupted`
          (`self.K2_EndAbility` :!label _label))
        (:`OnCancelled`
          (goto _label))
        (:`EventReceived`
          (`GameplayTask_WaitDelay.TaskWaitDelay` null 1.0
            (:`then`
              ;[1 0.002502 0.7689] GameplayCue
              (bind _output_get (set `self.GC Params` (`AbilitySystemBlueprintLibrary.MakeGameplayCueParameters` 0.0 0.0 (struct) (struct) (struct) (struct) (struct) (`MageAbilitySystemLibrary.GetMagicCircleLocation` null))))
              (`GameplayCueFunctionLibrary.AddGameplayCueOnActor` (`self.GetAvatarActorFromActorInfo`) (struct :`TagName` "GameplayCue.ThunderTronado") _output_get)
              (bind _outoverlappingactors (`MageAbilitySystemLibrary.GetLivingEnemyInCollisionShape` null _returnvalue (`|MakeArray` _returnvalue) (`MageAbilitySystemLibrary.GetMagicCircleLocation` null) "Capsule" true 0.0 (0.0 0.0 0.0) 10000.0 800.0))
              (for _array_element _outoverlappingactors
                (`MageAT_ApplyTargetRootMotionRadialForce.ApplyTargetRootMotionRadialForce` "None" _array_element (`MageAbilitySystemLibrary.GetMagicCircleLocation` null) null 200.0 (`self.Duration`) 1000.0 false false true null null false (struct) "MaintainLastRootMotionVelocity"
                  (:`then`
                    (`AbilityTask_WaitDelay.WaitDelay` (`self.Duration`)
                      (:`OnFinish`
                        (`GameplayCueFunctionLibrary.RemoveGameplayCueOnActor` (`self.GetAvatarActorFromActorInfo`) (struct :`TagName` "GameplayCue.ThunderTronado") (`self.GC Params`))
                        (`KismetSystemLibrary.PrintString` "REMOVE")
                        (`self.K2_EndAbility`)))))))
            (:`OnFinish`
              ;[1 0.03136 0] 伤害
              (bind _outoverlappingactors_2 (`MageAbilitySystemLibrary.GetLivingActorInCollisionShape` null (`|MakeArray` (`self.GetAvatarActorFromActorInfo`)) (`MageAbilitySystemLibrary.GetMagicCircleLocation` null) "Capsule" true 0.0 (200.0 200.0 200.0) 400.0 800.0))
              (for _array_element_2 _outoverlappingactors_2
                (bind _output_get_2 (set `self.TargetActor` _array_element_2))
                (`MageAbilitySystemLibrary.ApplyDamageEffect` (`self.MakeDamageEffectParamsFromClassDefault` _output_get_2))))))))))