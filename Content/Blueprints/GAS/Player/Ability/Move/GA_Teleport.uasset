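; Gameplay ability that teleports the mage a set distance along the horizontal components of its normalized velocity.
; It commits only when X or Y velocity is positive, so movement with neither component positive just ends the ability.
; After an unswept location change, it fires the Teleport gameplay cue at the origin, then ends and removes the cue.
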(event `self.K2_ActivateAbility`
  (bind (_returnvalue_x _returnvalue_y) (`KismetMathLibrary.BreakVector` (`KismetMathLibrary.Normal` (`Actor.GetVelocity` (`self.BP Mage`)))))
  (bind _asbp_mage (cast `/Game/Blueprints/Character/BP_Mage` (`self.GetAvatarActorFromActorInfo`))
    (:`then`
      (set `self.BP Mage` _asbp_mage)
      ;[1 1 1] 向速度朝向方向瞬移
      (set `self.Velocity X` _returnvalue_x)
      (set `self.Velocity Y` _returnvalue_y)
      (bind _returnvalue (`self.Has Velocity`))
      (if _returnvalue
        (bind _returnvalue_2 (`self.K2_CommitAbility`))
        (if _returnvalue_2
          (bind _output_get (set `self.Origin Location` (`Actor.K2_GetActorLocation` (`self.BP Mage`))))
          (bind (_bp_mage _returnvalue_3) (`self.Get Teleport Location` _output_get))
          (`Actor.K2_SetActorLocation` _bp_mage _returnvalue_3 false false)
          (`self.K2_AddGameplayCueWithParams` (struct :`TagName` "GameplayCue.Teleport") (`AbilitySystemBlueprintLibrary.MakeGameplayCueParameters` 0.0 0.0 (struct) (struct) (struct) (struct) (struct) _output_get))
          (`self.K2_EndAbility`)
          (`self.K2_RemoveGameplayCue` (struct :`TagName` "GameplayCue.Teleport"))
          (else
            (`self.K2_EndAbility`)))
        (else
          (`self.K2_EndAbility`))))
    (:`CastFailed`
      (`self.K2_EndAbility`))))

(fn `Get Teleport Location`
  (params (OriginLocation :type "Vector Structure"))
  (returns (`BP Mage` :type "/Game/Blueprints/Character/BP_Mage Object Reference") (ReturnValue :type "Vector Structure"))
  (bind _teleport_distance (`self.Teleport Distance`))
  (return (`self.BP Mage`) (+ OriginLocation (`KismetMathLibrary.MakeVector` (* (`self.Velocity X`) _teleport_distance) (* _teleport_distance (`self.Velocity Y`))))))

(fn `Has Velocity`
  (returns (ReturnValue :type Boolean))
  (return (or (> (`self.Velocity X`) 0.0) (> (`self.Velocity Y`) 0.0))))