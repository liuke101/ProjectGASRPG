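; BP_Mage is the mage character Blueprint, built from modular body meshes with a socketed weapon.
; An attribute-change listener started on BeginPlay copies new values into max walk speed.
; The CombatInterface facing event feeds MotionWarping's FacingTarget so root-motion skill montages turn toward enemies.
; Construction makes body parts follow the main mesh's pose and configures custom depth stencil for outlines, though Shoulder never gets custom depth enabled.
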(event `self.ReceiveBeginPlay`
  (`parent.ReceiveBeginPlay`)
  (bind (_asynctaskproxy _attribute _newvalue) (`AbilityAsync_WaitAttributeChanged.WaitForAttributeChanged` null (struct :`AttributeName` "MoveSpeed" :`Attribute` "/Script/ProjectGASRPG.MageAttributeSet:MoveSpeed" :`AttributeOwner` "/Script/CoreUObject.Class'\"/Script/ProjectGASRPG.MageAttributeSet\"'"))
    (:`Changed`
      (set `CharacterMovementComponent.MaxWalkSpeed` _newvalue (`self.CharacterMovement`)))))

(event `self.ReceiveTick`
  (params (DeltaSeconds :type "Float (single-precision)"))
  (`parent.ReceiveTick` DeltaSeconds))

(event `CombatInterface.UpdateFacingTarget`
  (params (TargetLocation :type "Vector Structure (by ref)"))
  ;[1 0.6164 0.2701] MotionWarping:释放技能时，使Montage面向敌人(动画必须开启根运动)
  ;;[0.5569 0.9661 1] CombatInterface
  (`MotionWarpingComponent.AddOrUpdateWarpTargetFromLocation` (`self.MotionWarping`) "FacingTarget" TargetLocation))

(fn `UserConstructionScript`
  (bind _weapon (`self.Weapon`))
  ;[1 1 1] Attach武器
  (`SceneComponent.K2_AttachToComponent` (`self.Weapon`) (`self.FillerMesh`) (`self.WeaponAttachSocket`) "SnapToTarget" "SnapToTarget" "SnapToTarget" true)
  ;[1 1 1] 模块化角色
  (`SkinnedMeshComponent.SetLeaderPoseComponent` (`.Chest` (`self.Modular Mesh`)) (`self.Mesh`) false false)
  (`SkinnedMeshComponent.SetLeaderPoseComponent` (`.Boots` (`self.Modular Mesh`)) (`self.Mesh`) false false)
  (`SkinnedMeshComponent.SetLeaderPoseComponent` (`.Legs` (`self.Modular Mesh`)) (`self.Mesh`) false false)
  (`SkinnedMeshComponent.SetLeaderPoseComponent` (`.Helmet` (`self.Modular Mesh`)) (`self.Mesh`) false false)
  (`SkinnedMeshComponent.SetLeaderPoseComponent` (`.Hands` (`self.Modular Mesh`)) (`self.Mesh`) false false)
  (`SkinnedMeshComponent.SetLeaderPoseComponent` (`.Back` (`self.Modular Mesh`)) (`self.Mesh`) false false)
  (`SkinnedMeshComponent.SetLeaderPoseComponent` (`self.Modular Mesh`) (`self.Mesh`) false false)
  (`SkinnedMeshComponent.SetLeaderPoseComponent` (`.Shoulder` (`self.Modular Mesh`)) (`self.Mesh`) false false)
  ;[1 1 1] 深度缓冲，用于描边
  (`PrimitiveComponent.SetRenderCustomDepth` _weapon true)
  (`PrimitiveComponent.SetRenderCustomDepth` (`.Chest` (`self.Modular Mesh`)) true)
  (`PrimitiveComponent.SetRenderCustomDepth` (`.Boots` (`self.Modular Mesh`)) true)
  (`PrimitiveComponent.SetRenderCustomDepth` (`.Legs` (`self.Modular Mesh`)) true)
  (`PrimitiveComponent.SetRenderCustomDepth` (`.Helmet` (`self.Modular Mesh`)) true)
  (`PrimitiveComponent.SetRenderCustomDepth` (`.Hands` (`self.Modular Mesh`)) true)
  (`PrimitiveComponent.SetRenderCustomDepth` (`.Back` (`self.Modular Mesh`)) true)
  (`PrimitiveComponent.SetRenderCustomDepth` (`self.Modular Mesh`) true)
  (`PrimitiveComponent.SetCustomDepthStencilValue` _weapon 0)
  (`PrimitiveComponent.SetCustomDepthStencilValue` (`.Chest` (`self.Modular Mesh`)) 0)
  (`PrimitiveComponent.SetCustomDepthStencilValue` (`.Boots` (`self.Modular Mesh`)) 0)
  (`PrimitiveComponent.SetCustomDepthStencilValue` (`.Legs` (`self.Modular Mesh`)) 0)
  (`PrimitiveComponent.SetCustomDepthStencilValue` (`.Helmet` (`self.Modular Mesh`)) 0)
  (`PrimitiveComponent.SetCustomDepthStencilValue` (`.Hands` (`self.Modular Mesh`)) 0)
  (`PrimitiveComponent.SetCustomDepthStencilValue` (`.Back` (`self.Modular Mesh`)) 0)
  (`PrimitiveComponent.SetCustomDepthStencilValue` (`self.Modular Mesh`) 0)
  (`PrimitiveComponent.SetCustomDepthStencilValue` (`.Shoulder` (`self.Modular Mesh`)) 0))